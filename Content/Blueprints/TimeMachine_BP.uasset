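; TimeMachine_BP is a damageable objective actor whose destruction ends the game.
; HPManagement subtracts incoming damage and updates a text render HP readout, which the construction script initializes; lethal damage calls GameOver on the main character and destroys the actor.
; BeginPlay caches the character and enemy spawner, though the spawner's SpecialWave check is unconnected.
; The box overlap only prints a debug message when the player enters.
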(event `self.ReceiveBeginPlay`
  (bind _returnvalue (`GameplayStatics.GetActorOfClass` "/Game/Blueprints/MainCharacter_BP.MainCharacter_BP_C"))
  (set `self.PlayerRef` _returnvalue)
  (bind _returnvalue_2 (`GameplayStatics.GetActorOfClass` "/Game/Blueprints/Enemies/EnemySpawner_MasterBP.EnemySpawner_MasterBP_C"))
  (set `self.SpawnerRef` _returnvalue_2))

(event `/Game/Blueprints/Core/HPManagement_Interface.HPManagement`
  (params (DMG :type "Float (single-precision)"))
  (bind _returnvalue (- (`self.HPCurrent`) DMG))
  (if (> _returnvalue 0.0)
    (bind _output_get (set `self.HPCurrent` _returnvalue))
    (`TextRenderComponent.K2_SetText` (`self.TextRender`) (`KismetTextLibrary.Conv_DoubleToText` _output_get "HalfToEven"))
    (else
      (`/Game/Blueprints/MainCharacter_BP.GameOver` (`self.PlayerRef`))
      (`self.K2_DestroyActor`))))

(event `self.Box.OnComponentBeginOverlap`
  (params (OverlappedComponent :type "PrimitiveComponent Object Reference") (OtherActor :type "Actor Object Reference") (OtherComp :type "PrimitiveComponent Object Reference") (OtherBodyIndex :type Integer) (bFromSweep :type Boolean) (SweepResult :type "HitResult Structure (by ref)"))
  (if (`self.ActorHasTag` OtherActor "Player")
    (`KismetSystemLibrary.PrintString` "PlayerInRange")))

(fn `UserConstructionScript`
  (`TextRenderComponent.K2_SetText` (`self.TextRender`) (`KismetTextLibrary.Conv_DoubleToText` (`self.HPCurrent`) "HalfToEven")))