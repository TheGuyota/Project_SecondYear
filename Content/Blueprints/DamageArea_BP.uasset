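; DamageArea_BP is a temporary area hazard that deals periodic damage to actors inside its box, then destroys itself.
; Overlap events track actors implementing HPManagement_Interface in an array, adding them on entry and removing them on exit.
; A looping one-second timer sends each tracked actor DMGInTime through HPManagementMessage, until a Duration timer clears it.
; The construction script sizes the box's X and Y extents from AreaOfDamage.
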(event `self.ReceiveBeginPlay`
  (bind _returnvalue (`KismetSystemLibrary.K2_SetTimerDelegate` (delegate `DamageOnTime`) 1.0 true))
  (set `self.DamageHandle` _returnvalue)
  (`KismetSystemLibrary.K2_SetTimerDelegate` (delegate `StopDamage`) (`self.Duration`)))

(event `DamageOnTime`
  (for _array_element (`self.ActorToDamage`)
    (message `/Game/Blueprints/Core/HPManagement_Interface.HPManagement` _array_element (`self.DMGInTime`))))

(event `StopDamage`
  (`KismetSystemLibrary.K2_ClearAndInvalidateTimerHandle` (`self.DamageHandle`))
  (`self.K2_DestroyActor`))

(event `self.Box.OnComponentBeginOverlap`
  (params (OverlappedComponent :type "PrimitiveComponent Object Reference") (OtherActor :type "Actor Object Reference") (OtherComp :type "PrimitiveComponent Object Reference") (OtherBodyIndex :type Integer) (bFromSweep :type Boolean) (SweepResult :type "HitResult Structure (by ref)"))
  (if (`KismetSystemLibrary.DoesImplementInterface` OtherActor "/Game/Blueprints/Core/HPManagement_Interface.HPManagement_Interface_C")
    (`KismetArrayLibrary.Array_Add` (`self.ActorToDamage`) OtherActor)))

(event `self.Box.OnComponentEndOverlap`
  (params (OverlappedComponent :type "PrimitiveComponent Object Reference") (OtherActor :type "Actor Object Reference") (OtherComp :type "PrimitiveComponent Object Reference") (OtherBodyIndex :type Integer))
  (bind _actortodamage (`self.ActorToDamage`))
  (if (`KismetSystemLibrary.DoesImplementInterface` OtherActor "/Game/Blueprints/Core/HPManagement_Interface.HPManagement_Interface_C")
    (`KismetArrayLibrary.Array_Remove` _actortodamage (`KismetArrayLibrary.Array_Find` _actortodamage OtherActor))))

(fn `UserConstructionScript`
  (bind _areaofdamage (`self.AreaOfDamage`))
  (`BoxComponent.SetBoxExtent` (`self.Box`) (`KismetMathLibrary.MakeVector` _areaofdamage _areaofdamage) true))