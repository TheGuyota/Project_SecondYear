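; Fire pit actor that creates a temporary area of fire dealing periodic damage.
; CreateFirePit spawns a Niagara fire effect at the given location and starts a looping one-second damage timer plus a FireDuration timer.
; Each tick sphere-traces around the effect and sends HPManagement_Interface damage, skipping only consecutive duplicate hits on the same actor.
; When the duration ends, the effect and actor are destroyed.
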(event `CreateFirePit`
  (params (FireLocation :type "Vector Structure"))
  (bind _returnvalue (`NiagaraFunctionLibrary.SpawnSystemAtLocation` "/Game/SFX/Particles/Fire_NS.Fire_NS" FireLocation (struct) (21.0 20.0 1.0)))
  (set `self.ActiveFireEffects` _returnvalue)
  (bind _returnvalue_2 (`KismetSystemLibrary.K2_SetTimerDelegate` (delegate `StartFireDamage`) 1.0 true))
  (set `self.FireDamageHandle` _returnvalue_2)
  (`KismetSystemLibrary.K2_SetTimerDelegate` (delegate `StopFire`) (`self.FireDuration`)))

(event `StartFireDamage`
  (bind _returnvalue (`SceneComponent.K2_GetComponentLocation` (`self.ActiveFireEffects`)))
  (set `self.LastHitActor` null)
  (bind _outhits (`KismetSystemLibrary.SphereTraceMulti` :`Start` _returnvalue :`End` _returnvalue :`Radius` 220.0 :`TraceChannel` "TraceTypeQuery5" :`DrawTime` 0.5))
  (for _array_element _outhits
    (bind (_bblockinghit _binitialoverlap _time _distance _location _impactpoint _normal _impactnormal _physmat _hitactor _hitcomponent) (`GameplayStatics.BreakHitResult` _array_element))
    (if (`KismetSystemLibrary.DoesImplementInterface` _hitactor "/Game/Blueprints/Core/HPManagement_Interface.HPManagement_Interface_C")
      (if (not (== _hitactor (`self.LastHitActor`)))
        (set `self.LastHitActor` _hitactor)
        (message `/Game/Blueprints/Core/HPManagement_Interface.HPManagement` _hitactor (`self.FirePitDamage`) _hitcomponent)))))

(event `StopFire`
  (`KismetSystemLibrary.PrintString` "FireEnded")
  (`ActorComponent.K2_DestroyComponent` (`self.ActiveFireEffects`))
  (`self.K2_DestroyActor`))

(fn `UserConstructionScript`)