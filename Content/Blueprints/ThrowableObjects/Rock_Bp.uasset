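; Rock_Bp is a throwable rock that deals damage on contact and then removes itself.
; When its sphere overlaps an actor without the Player tag, it sends DMG through HPManagement_Interface if that actor implements it.
; The rock destroys itself after any such overlap, damaged or not, and also on any Hit event.
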(event `self.Sphere.OnComponentBeginOverlap`
  (params (OverlappedComponent :type "PrimitiveComponent Object Reference") (OtherActor :type "Actor Object Reference") (OtherComp :type "PrimitiveComponent Object Reference") (OtherBodyIndex :type Integer) (bFromSweep :type Boolean) (SweepResult :type "HitResult Structure (by ref)"))
  (if (not (`self.ActorHasTag` OtherActor "Player"))
    (if (`KismetSystemLibrary.DoesImplementInterface` OtherActor "/Game/Blueprints/Core/HPManagement_Interface.HPManagement_Interface_C")
      (message `/Game/Blueprints/Core/HPManagement_Interface.HPManagement` OtherActor (`self.DMG`))
      (`self.K2_DestroyActor`)
      (else
        (`self.K2_DestroyActor`)))))

(event `self.ReceiveHit`
  (params (MyComp :type "PrimitiveComponent Object Reference") (Other :type "Actor Object Reference") (OtherComp :type "PrimitiveComponent Object Reference") (bSelfMoved :type Boolean) (HitLocation :type "Vector Structure") (HitNormal :type "Vector Structure") (NormalImpulse :type "Vector Structure") (Hit :type "HitResult Structure (by ref)"))
  (`self.K2_DestroyActor`))

(fn `UserConstructionScript`
  (`parent.UserConstructionScript`))