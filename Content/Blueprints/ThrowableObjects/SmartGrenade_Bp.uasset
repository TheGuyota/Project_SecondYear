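; Homing grenade pawn that chases an enemy and deals area damage on arrival.
; An overlap on its detection range stores the actor as the target and, if it is tagged Enemy, starts an AI move toward it.
; On arrival, a debug-drawn multi sphere trace sends damage to any hit actor implementing the HP management interface, regardless of tag, then the grenade destroys itself.
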(event `self.DetectionRange.OnComponentBeginOverlap`
  (params (OverlappedComponent :type "PrimitiveComponent Object Reference") (OtherActor :type "Actor Object Reference") (OtherComp :type "PrimitiveComponent Object Reference") (OtherBodyIndex :type Integer) (bFromSweep :type Boolean) (SweepResult :type "HitResult Structure (by ref)"))
  (bind _returnvalue (`self.K2_GetActorLocation`))
  (set `self.TargetedEnemy` OtherActor)
  (`KismetSystemLibrary.PrintString` "Print OK")
  (if (`self.ActorHasTag` OtherActor "Enemy")
    (`KismetSystemLibrary.PrintString` "Tag OK")
    (`|AIMoveTo` self (0.0 0.0 0.0) (`self.TargetedEnemy`) 10.0
      (:`OnSuccess`
        (bind _outhits (`KismetSystemLibrary.SphereTraceMulti` :`Start` _returnvalue :`End` _returnvalue :`Radius` 300.0 :`TraceChannel` "TraceTypeQuery5" :`DrawDebugType` "ForDuration" :`DrawTime` 0.2))
        (for _array_element _outhits
          (bind (_bblockinghit _binitialoverlap _time _distance _location _impactpoint _normal _impactnormal _physmat _hitactor) (`GameplayStatics.BreakHitResult` _array_element))
          (if (`KismetSystemLibrary.DoesImplementInterface` _hitactor "/Game/Blueprints/Core/HPManagement_Interface.HPManagement_Interface_C")
            (message `/Game/Blueprints/Core/HPManagement_Interface.HPManagement` _hitactor (`self.DMG`))))
        (`self.K2_DestroyActor`)))))

(fn `UserConstructionScript`)