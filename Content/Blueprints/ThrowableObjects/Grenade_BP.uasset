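; Timed grenade that explodes after a fuse set on BeginPlay, then destroys itself.
; The explosion runs a zero-length multi sphere trace at its location, with debug drawing on, using the Range radius.
; Each hit whose actor implements HPManagement_Interface receives point damage, credited to the MainCharacter_BP found at BeginPlay as damage causer.
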(event `self.ReceiveBeginPlay`
  (`KismetSystemLibrary.K2_SetTimerDelegate` (delegate `Explode`) (`self.Timer`))
  (bind _returnvalue (`GameplayStatics.GetActorOfClass` "/Game/Blueprints/MainCharacter_BP.MainCharacter_BP_C")))

(event `Explode`
  (bind _returnvalue (`self.K2_GetActorLocation`))
  (bind _outhits (`KismetSystemLibrary.SphereTraceMulti` :`Start` _returnvalue :`End` _returnvalue :`Radius` (`self.Range`) :`TraceChannel` "TraceTypeQuery5" :`DrawDebugType` "ForDuration" :`DrawTime` 0.2))
  (for _array_element _outhits
    (bind (_bblockinghit _binitialoverlap _time _distance _location _impactpoint _normal _impactnormal _physmat _hitactor _hitcomponent _hitbonename _hititem _elementindex _faceindex _tracestart) (`GameplayStatics.BreakHitResult` _array_element))
    (if (`KismetSystemLibrary.DoesImplementInterface` _hitactor "/Game/Blueprints/Core/HPManagement_Interface.HPManagement_Interface_C")
      (`GameplayStatics.ApplyPointDamage` _hitactor (`self.DMG`) _tracestart _array_element null (stale `self.ReceiveBeginPlay` _returnvalue))))
  (`self.K2_DestroyActor`))

(fn `UserConstructionScript`
  (`parent.UserConstructionScript`))