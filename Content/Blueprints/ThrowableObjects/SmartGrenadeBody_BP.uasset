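; Smart grenade projectile body that seeks an actor tagged "Enemy" and deals area damage when it reaches one.
; After launch it arms its contact sphere, halts its projectile movement, and rises on a looping timer before enabling the detection box.
; An enemy entering the box becomes the target, which the grenade homes toward by timed location lerps after a short delay.
; Sphere contact triggers a radial trace, sends damage through HPManagement_Interface, and destroys the grenade.
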(event `self.ReceiveBeginPlay`
  (`KismetSystemLibrary.Delay` 2.0)
  (`PrimitiveComponent.SetCollisionEnabled` (`self.Sphere2`) "QueryOnly")
  (`KismetSystemLibrary.Delay` 1.0)
  (`self.StartAllLogic`))

(event `StartAllLogic`
  (`KismetSystemLibrary.K2_SetTimerDelegate` (delegate `StopAllLogic`) 1.5))

(event `StopAllLogic`
  (`MovementComponent.StopMovementImmediately` (`self.ProjectileMovement`))
  (bind _returnvalue (`KismetSystemLibrary.K2_SetTimerDelegate` (delegate `GetUp`) 0.1 true))
  (set `self.GetUpHandle` _returnvalue)
  (`KismetSystemLibrary.K2_SetTimerDelegate` (delegate `StopGetUp`) 2.5))

(event `GetUp`
  (bind (_returnvalue_x _returnvalue_y _returnvalue_z) (`KismetMathLibrary.BreakVector` (`self.K2_GetActorLocation`)))
  (`self.K2_SetActorLocation` (`KismetMathLibrary.MakeVector` _returnvalue_x _returnvalue_y (`KismetMathLibrary.Lerp` _returnvalue_z (+ _returnvalue_z 200.0) 0.04))))

(event `StopGetUp`
  (`KismetSystemLibrary.K2_ClearAndInvalidateTimerHandle` (`self.GetUpHandle`))
  (`PrimitiveComponent.SetCollisionEnabled` (`self.Box`) "QueryOnly"))

(event `self.Box.OnComponentBeginOverlap`
  (params (OverlappedComponent :type "PrimitiveComponent Object Reference") (OtherActor :type "Actor Object Reference") (OtherComp :type "PrimitiveComponent Object Reference") (OtherBodyIndex :type Integer) (bFromSweep :type Boolean) (SweepResult :type "HitResult Structure (by ref)"))
  (if (`self.ActorHasTag` OtherActor "Enemy")
    (set `self.Target` OtherActor)
    (`KismetSystemLibrary.Delay` 2.0)
    (`KismetSystemLibrary.K2_SetTimerDelegate` (delegate `ReachTarget`) 0.05 true)))

(event `self.Sphere2.OnComponentBeginOverlap`
  (params (OverlappedComponent :type "PrimitiveComponent Object Reference") (OtherActor :type "Actor Object Reference") (OtherComp :type "PrimitiveComponent Object Reference") (OtherBodyIndex :type Integer) (bFromSweep :type Boolean) (SweepResult :type "HitResult Structure (by ref)"))
  (bind _returnvalue (`self.K2_GetActorLocation`))
  (if (`self.ActorHasTag` OtherActor "Enemy")
    (bind _outhits (`KismetSystemLibrary.SphereTraceMulti` _returnvalue _returnvalue 300.0 "TraceTypeQuery5"))
    (for _array_element _outhits
      (bind (_bblockinghit _binitialoverlap _time _distance _location _impactpoint _normal _impactnormal _physmat _hitactor _hitcomponent) (`GameplayStatics.BreakHitResult` _array_element))
      (`/Engine/EditorBlueprintResources/StandardMacros.IsValid` _hitactor
        (:`Is Valid`
          (if (`KismetSystemLibrary.DoesImplementInterface` _hitactor "/Game/Blueprints/Core/HPManagement_Interface.HPManagement_Interface_C")
            (if (not (== _hitactor (`self.LastHitActor`)))
              (set `self.LastHitActor` _hitactor)
              (message `/Game/Blueprints/Core/HPManagement_Interface.HPManagement` _hitactor (`self.BodyDMG`) _hitcomponent))
            (else
              (`self.K2_DestroyActor`))))
        (:`Is Not Valid`
          (`self.K2_DestroyActor`))))
    (`self.K2_DestroyActor`)))

(event `ReachTarget`
  (bind _target (`self.Target`))
  (`/Engine/EditorBlueprintResources/StandardMacros.IsValid` _target
    (:`Is Valid`
      (`self.K2_SetActorLocation` (`KismetMathLibrary.VLerp` (`self.K2_GetActorLocation`) (`self.K2_GetActorLocation` _target) 0.08)))
    (:`Is Not Valid`
      (`self.K2_DestroyActor`))))

(fn `UserConstructionScript`
  (`PrimitiveComponent.SetCollisionEnabled` (`self.Box`) "NoCollision"))