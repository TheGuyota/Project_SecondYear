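; Smart throwable grenade, marked work in progress, that homes in on an enemy and explodes near it.
; FlyingRange overlaps lock the first "Enemy"-tagged actor, which Tick chases by setting Sphere velocity toward it.
; Other overlaps without a target trigger, after a delay, a Timeline lift that leaves the grenade hovering without physics.
; When the target enters ExplosionRange, a multi-sphere trace sends damage through HPManagement_Interface and the grenade destroys itself.
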(event `self.ReceiveTick`
  (params (DeltaSeconds :type "Float (single-precision)"))
  ;[1 0 0] ANCORA IN FASE DI ELABORAZIONE
  (`/Engine/EditorBlueprintResources/StandardMacros.IsValid` (`self.EnemyRef`)
    (:`Is Valid`
      (`PrimitiveComponent.SetPhysicsLinearVelocity` (`self.Sphere`) (* (- (`self.K2_GetActorLocation` (`self.EnemyRef`)) (`self.K2_GetActorLocation`)) 2.5) false "None"))))

(event `self.ExplosionRange.OnComponentBeginOverlap`
  (params (OverlappedComponent :type "PrimitiveComponent Object Reference") (OtherActor :type "Actor Object Reference") (OtherComp :type "PrimitiveComponent Object Reference") (OtherBodyIndex :type Integer) (bFromSweep :type Boolean) (SweepResult :type "HitResult Structure (by ref)"))
  (bind _returnvalue (`self.K2_GetActorLocation`))
  ;[1 0 0] ANCORA IN FASE DI ELABORAZIONE
  (if (== OtherActor (`self.EnemyRef`))
    (bind _outhits (`KismetSystemLibrary.SphereTraceMulti` :`Start` _returnvalue :`End` _returnvalue :`Radius` (`self.Range`) :`TraceChannel` "TraceTypeQuery5" :`DrawDebugType` "ForDuration" :`DrawTime` 0.2))
    (for _array_element _outhits
      (bind (_bblockinghit _binitialoverlap _time _distance _location _impactpoint _normal _impactnormal _physmat _hitactor) (`GameplayStatics.BreakHitResult` _array_element))
      (if (`KismetSystemLibrary.DoesImplementInterface` _hitactor "/Game/Blueprints/Core/HPManagement_Interface.HPManagement_Interface_C")
        (message `/Game/Blueprints/Core/HPManagement_Interface.HPManagement` _hitactor (`self.DMG`))))
    (`self.K2_DestroyActor`)))

(event `self.FlyingRange.OnComponentBeginOverlap`
  (params (OverlappedComponent :type "PrimitiveComponent Object Reference") (OtherActor :type "Actor Object Reference") (OtherComp :type "PrimitiveComponent Object Reference") (OtherBodyIndex :type Integer) (bFromSweep :type Boolean) (SweepResult :type "HitResult Structure (by ref)"))
  (bind (_returnvalue_x _returnvalue_y _returnvalue_z) (`KismetMathLibrary.BreakVector` (`self.K2_GetActorLocation`)))
  (bind _sphere (`self.Sphere`))
  ;[1 0 0] ANCORA IN FASE DI ELABORAZIONE
  (`/Engine/EditorBlueprintResources/StandardMacros.IsValid` (`self.EnemyRef`)
    (:`Is Not Valid`
      (if (`self.ActorHasTag` OtherActor "Enemy")
        (set `self.EnemyRef` OtherActor)
        (else
          (`KismetSystemLibrary.Delay` 2.0)
          (if (not (`self.bStandingInAir`))
            (bind (_direction _zvalue) (`Timeline|StandInAir` :!via `PlayFromStart`)
              (:`Update`
                (bind _output_get (set `self.StartingZ` _returnvalue_z))
                (`self.K2_SetActorLocation` (`KismetMathLibrary.MakeVector` _returnvalue_x _returnvalue_y (+ _output_get _zvalue))))
              (:`Finished`
                (`MovementComponent.StopMovementImmediately` (`self.ProjectileMovement`))
                (`PrimitiveComponent.SetEnableGravity` _sphere false)
                (`PrimitiveComponent.SetSimulatePhysics` _sphere false)
                (set `ProjectileMovementComponent.ProjectileGravityScale` 0.0 (`self.ProjectileMovement`))
                (set `self.bStandingInAir` true)))))))))

(fn `UserConstructionScript`
  (`parent.UserConstructionScript`))