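; Base Blueprint for a mobile platform that moves up and down while switched on by a button interaction.
; ButtonInteraction toggles IsActive and calls MovePlatforms, which plays a Movement timeline and then a Reverse timeline to drive the static mesh's relative Z, with a short delay before each.
; MovePlatforms calls itself when Reverse finishes, so the cycle repeats until that check finds IsActive false, and switching off does not interrupt a cycle already running.
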(event `/Game/Blueprints/Core/ButtonInteraction_Interface.ButtonInteraction`
  (set `self.bIsActive` (not (`self.bIsActive`)))
  (`self.MovePlatforms`))

(event `MovePlatforms`
  (if (`self.bIsActive`)
    (`KismetSystemLibrary.Delay` 1.0)
    (bind (_direction _zvalue) (`Timeline|Movement` :!via `PlayFromStart`)
      (:`Update`
        (`SceneComponent.K2_SetRelativeLocation` (`self.StaticMesh`) (`KismetMathLibrary.MakeVector` 0.0 0.0 _zvalue) false false))
      (:`Finished`
        (`KismetSystemLibrary.Delay` 1.0)
        (bind (_direction_2 _zvaluereverse) (`Timeline|Reverse` :!via `PlayFromStart`)
          (:`Update`
            (`SceneComponent.K2_SetRelativeLocation` (`self.StaticMesh`) (`KismetMathLibrary.MakeVector` 0.0 0.0 _zvaluereverse) false false))
          (:`Finished`
            (`self.MovePlatforms`)))))))

(fn `UserConstructionScript`)