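; Rifle weapon Blueprint that fires a hitscan shot from the shooter's camera when its Action event is called.
; Action plays the fire sound and line traces along the camera's forward vector, ignoring the shooter.
; It also spawns a FirstPersonProjectile offset from ProjectileSpawn on every shot, independent of the trace result.
; Hit actors tagged "Enemy" trigger a 2D hit-marker sound and receive point damage from the DMG variable.
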(event `/Game/Blueprints/Core/WeaponAction_Interface.Action`
  (params (CameraLocation :type "Vector Structure") (CameraRotation :type "Rotator Structure") (ShooterRef :type "/Game/Blueprints/MainCharacter_BP Object Reference"))
  (`GameplayStatics.PlaySoundAtLocation` "/Game/SoundEffects/WeaponFire.WeaponFire" (`SceneComponent.RelativeLocation` (`self.ProjectileSpawn`)) (struct) 1.0 1.0 0.0 null null null)
  (bind _outhit (`KismetSystemLibrary.LineTraceSingle` CameraLocation (+ CameraLocation (* (`KismetMathLibrary.GetForwardVector` CameraRotation) 15000.0)) "TraceTypeQuery3" false (`|MakeArray` ShooterRef :!type "Actor Object Reference") "None" true (struct :`R` 1.0 :`A` 1.0) (struct :`G` 1.0 :`A` 1.0) 1.5))
  (`|SpawnActorFromClass` "/Game/FirstPersonBP/Blueprints/FirstPersonProjectile.FirstPersonProjectile_C" (`KismetMathLibrary.MakeTransform` (+ (`SceneComponent.K2_GetComponentLocation` (`self.ProjectileSpawn`)) (`KismetMathLibrary.GreaterGreater_VectorRotator` (100.0 0.0 -10.0) CameraRotation)) CameraRotation) "Undefined" "OverrideRootScale" null null)
  (bind (_bblockinghit _binitialoverlap _time _distance _location _impactpoint _normal _impactnormal _physmat _hitactor _hitcomponent _hitbonename _hititem _elementindex _faceindex _tracestart) (`GameplayStatics.BreakHitResult` _outhit))
  (`/Engine/EditorBlueprintResources/StandardMacros.IsValid` _hitactor
    (:`Is Valid`
      (if (`self.ActorHasTag` _hitactor "Enemy")
        (`GameplayStatics.PlaySound2D` "/Game/SoundEffects/HItMarker.HItMarker" 1.0 1.0 0.0 null null)
        (`GameplayStatics.ApplyPointDamage` _hitactor (`self.DMG`) _tracestart _outhit)))))

(fn `UserConstructionScript`)