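; Master weapon Blueprint that holds a damage value and scales it with the player's level.
; The UpdateDamage event calls a function that, for positive levels, compounds DMG by 8% once per level above the stored LastPlayerLvl.
; That function then stores the level difference, not the current level, in LastPlayerLvl.
; Tick prints the current damage every frame as debug output.
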(event `self.ReceiveTick`
  (params (DeltaSeconds :type "Float (single-precision)"))
  (`KismetSystemLibrary.PrintString` (`KismetStringLibrary.Concat_StrStr` "ACTUAL WEAPON DAMAGE : " (`KismetStringLibrary.Conv_DoubleToString` (`self.DMG`))) true true (struct :`G` 0.66 :`B` 1.0 :`A` 1.0) 0.0))

(event `/Game/Blueprints/Core/WeaponAction_Interface.UpdateDamage`
  (params (PlayerLvl :type Integer))
  (`self.UpdateWeaponDamageBasedOnPlayerLevel` PlayerLvl))

(fn `UpdateWeaponDamageBasedOnPlayerLevel`
  (params (PlayerLvl :type Integer))
  (bind _dmg (`self.DMG`))
  (bind _returnvalue (- PlayerLvl (`self.LastPlayerLvl`)))
  (if (> PlayerLvl 0)
    (for _ (range 1 (+ _returnvalue 1))
      (set `self.DMG` (+ _dmg (* _dmg 0.08))))
    (set `self.LastPlayerLvl` _returnvalue)
    (return)
    (else
      (return))))

(fn `UserConstructionScript`)