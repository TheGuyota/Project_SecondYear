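; Lancia_BP is a melee lance weapon whose Action event performs a thrust attack for the shooter.
; An AnimationEnded flag blocks repeat attacks while the Attack timeline drives the actor's relative roll.
; When the timeline finishes, a short line trace from the camera, ignoring the shooter, applies multiplier-scaled point damage to hit actors implementing HPManagement_Interface.
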(event `/Game/Blueprints/Core/WeaponAction_Interface.Action`
  (params (CameraLocation :type "Vector Structure") (CameraRotation :type "Rotator Structure") (ShooterRef :type "/Game/Blueprints/MainCharacter_BP Object Reference") (DMGMultiplier :type "Float (single-precision)"))
  (if (`self.AnimationEnded`)
    (set `self.AnimationEnded` false)
    (bind (_direction _xvalue) (`Timeline|Attack` :!via `PlayFromStart`)
      (:`Update`
        (`self.K2_SetActorRelativeRotation` (`KismetMathLibrary.MakeRotator` _xvalue)))
      (:`Finished`
        (set `self.AnimationEnded` true)
        (bind _outhit (`KismetSystemLibrary.LineTraceSingle` CameraLocation (+ CameraLocation (* (`KismetMathLibrary.GetForwardVector` CameraRotation) 500.0)) "TraceTypeQuery3" false (`|MakeArray` ShooterRef :!type "Actor Object Reference") "None" true (struct :`R` 1.0 :`A` 1.0) (struct :`G` 1.0 :`A` 1.0) 1.5))
        (bind (_bblockinghit _binitialoverlap _time _distance _location _impactpoint _normal _impactnormal _physmat _hitactor _hitcomponent _hitbonename _hititem _elementindex _faceindex _tracestart) (`GameplayStatics.BreakHitResult` _outhit))
        (if (`KismetSystemLibrary.DoesImplementInterface` _hitactor "/Game/Blueprints/Core/HPManagement_Interface.HPManagement_Interface_C")
          (`GameplayStatics.ApplyPointDamage` _hitactor (* (`self.DMG`) DMGMultiplier) _tracestart _outhit null ShooterRef))))))

(fn `UserConstructionScript`
  (`parent.UserConstructionScript`))