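; Collectible time machine component pickup that the player gathers by overlapping its box.
; On overlap with a Player-tagged actor, it increments the main character's component count if below the cap of three and updates the component icons.
; It then clears the spawner manager's spawned flag and destroys itself.
; Each tick, its text label turns to face the player with pitch held flat.
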(event `self.ReceiveBeginPlay`
  (bind _returnvalue (`GameplayStatics.GetActorOfClass` "/Game/Blueprints/MainCharacter_BP.MainCharacter_BP_C"))
  (set `self.PlayerRef` _returnvalue))

(event `self.Box.OnComponentBeginOverlap`
  (params (OverlappedComponent :type "PrimitiveComponent Object Reference") (OtherActor :type "Actor Object Reference") (OtherComp :type "PrimitiveComponent Object Reference") (OtherBodyIndex :type Integer) (bFromSweep :type Boolean) (SweepResult :type "HitResult Structure (by ref)"))
  (bind _playerref (`self.PlayerRef`))
  (if (`self.ActorHasTag` OtherActor "Player")
    (if (< (`/Game/Blueprints/MainCharacter_BP.TimeMachineComponents` (`self.PlayerRef`)) 3)
      (`/Engine/EditorBlueprintResources/StandardMacros.IncrementInt` (`/Game/Blueprints/MainCharacter_BP.TimeMachineComponents` _playerref)
        (:`  `
          (`/Game/Blueprints/MainCharacter_BP.UpdateTimeMachineComponentIcons` _playerref true (`self.Icon`))
          (set `/Game/Blueprints/SpawnManager_MasterBP.isTimeMachineComponentSpawned` false (`self.SpawnerManagerRef`))
          (`self.K2_DestroyActor`))))))

(event `self.ReceiveTick`
  (params (DeltaSeconds :type "Float (single-precision)"))
  (bind _playerref (`self.PlayerRef`))
  (bind (_returnvalue_roll _returnvalue_pitch _returnvalue_yaw) (`KismetMathLibrary.BreakRotator` (`KismetMathLibrary.FindLookAtRotation` (`SceneComponent.K2_GetComponentLocation` (`self.TextRender`)) (`self.K2_GetActorLocation` _playerref))))
  (`/Engine/EditorBlueprintResources/StandardMacros.IsValid` _playerref
    (:`Is Valid`
      (`SceneComponent.K2_SetWorldRotation` (`self.TextRender`) (`KismetMathLibrary.MakeRotator` _returnvalue_roll 0.0 _returnvalue_yaw) false false))))

(fn `UserConstructionScript`)