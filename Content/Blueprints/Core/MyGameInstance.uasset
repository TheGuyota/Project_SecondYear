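; Game Instance that holds a reference to the main character and provides a central function for changing its stats.
; On Init it waits briefly, then finds and caches the MainCharacter_BP actor.
; UpdateStat switches on a stat type to set current HP, walk speed or jump velocity on that cached character, then refreshes all of its HUD stats.
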(event `self.ReceiveInit`
  (`KismetSystemLibrary.Delay` 0.2)
  (bind _returnvalue (`GameplayStatics.GetActorOfClass` "/Game/Blueprints/MainCharacter_BP.MainCharacter_BP_C"))
  (set `self.PlayerRef` _returnvalue))

(fn `UpdateStat`
  (params (StatToUpdate :type "/Game/Blueprints/StatsTypes Enum" :default "NewEnumerator4") (NewValue :type "Float (double-precision)"))
  (switch `/Game/Blueprints/StatsTypes` StatToUpdate
    (:`NewEnumerator4`
      (set `/Game/Blueprints/MainCharacter_BP.HP_Current` NewValue (`self.PlayerRef`)))
    (:`NewEnumerator0`
      (set `CharacterMovementComponent.MaxWalkSpeed` NewValue (`Character.CharacterMovement` (`self.PlayerRef`))))
    (:`NewEnumerator1`
      (set `CharacterMovementComponent.JumpZVelocity` NewValue (`Character.CharacterMovement` (`self.PlayerRef`)))))
  (`/Game/Blueprints/MainCharacter_BP.UpdateHUDStats` (`self.PlayerRef`) "NewEnumerator3")
  (return))