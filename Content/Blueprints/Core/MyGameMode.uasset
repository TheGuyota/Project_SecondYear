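; Game mode that drives periodic time travel between three eras.
; A looping timer fires every TimeBetweenTimeTravel seconds, switching to a random era, calling TimeTravel and restarting a one-second countdown timer.
; SwitchToRandomEra always picks a different era from the current one, and also runs in the construction script to randomize the starting era.
; Tick prints the remaining countdown and current era on screen.
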(event `self.ReceiveTick`
  (params (DeltaSeconds :type "Float (single-precision)"))
  (`KismetSystemLibrary.PrintString` (`KismetStringLibrary.Concat_StrStr` "Time Remaining Before Time Travel : " (`KismetStringLibrary.Conv_DoubleToString` (`self.CountdownTimeRemaining`))) true true (struct :`G` 0.66 :`B` 1.0 :`A` 1.0) 0.0)
  (`KismetSystemLibrary.PrintString` (`KismetStringLibrary.Concat_StrStr` "Actual Era: " (`|GetEnumeratorNameAsString` (`self.ActualEra`))) true true (struct :`R` 1.0 :`A` 1.0) 0.0))

(event `self.ReceiveBeginPlay`
  (`KismetSystemLibrary.K2_SetTimerDelegate` (delegate `CicleMap`) (`self.TimeBetweenTimeTravel`) true)
  (set `self.CountdownTimeRemaining` (`self.TimeBetweenTimeTravel`) :!label _label)
  (bind _returnvalue (`KismetSystemLibrary.K2_SetTimerDelegate` (delegate `TimeTravelCountdown`) 1.0 true))
  (set `self.CountdownHandle` _returnvalue))

(event `TimeTravelCountdown`
  (`/Engine/EditorBlueprintResources/StandardMacros.DecrementFloat` (`self.CountdownTimeRemaining`)))

(event `CicleMap`
  (`KismetSystemLibrary.PrintString` "Time Travel!")
  (`self.SwitchToRandomEra`)
  (`self.TimeTravel`)
  (`KismetSystemLibrary.K2_ClearAndInvalidateTimerHandle` (`self.CountdownHandle`))
  (goto _label))

(fn `SwitchToRandomEra`
  (locals (EraToSet :type "/Game/Blueprints/TimeTypes Enum"))
  (switch `int` (`KismetMathLibrary.RandomIntegerInRange` 0 2)
    (:`0`
      (bind _output_get (set `local.EraToSet` "NewEnumerator0"))
      (if (`|EnumEquality` _output_get (`self.ActualEra`))
        (if (`KismetMathLibrary.RandomBool`)
          (set `self.ActualEra` "NewEnumerator1")
          (else
            (set `self.ActualEra` "NewEnumerator2")))
        (else
          (set `self.ActualEra` (`local.EraToSet`))
          (return))))
    (:`1`
      (bind _output_get_2 (set `local.EraToSet` "NewEnumerator1"))
      (if (`|EnumEquality` _output_get_2 (`self.ActualEra`))
        (if (`KismetMathLibrary.RandomBool`)
          (set `self.ActualEra` "NewEnumerator0")
          (else
            (set `self.ActualEra` "NewEnumerator2")))
        (else
          (set `self.ActualEra` (`local.EraToSet`))
          (return))))
    (:`2`
      (bind _output_get_3 (set `local.EraToSet` "NewEnumerator2"))
      (if (`|EnumEquality` _output_get_3 (`self.ActualEra`))
        (if (`KismetMathLibrary.RandomBool`)
          (set `self.ActualEra` "NewEnumerator0")
          (else
            (set `self.ActualEra` "NewEnumerator1")))
        (else
          (set `self.ActualEra` (`local.EraToSet`))
          (return)))))
  (return))

(fn `UserConstructionScript`
  (`self.SwitchToRandomEra`))