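; Wave manager that spawns enemies from EnemySpawner actors in escalating normal waves, with periodic timed special waves.
; Timers drive spawning; normal waves grow and target the player, while special waves target the time machine until spawning times out and all enemies die.
; Wave count sets the game stage for weighted enemy type picks and triggers TimeMachineComponent spawns at random points.
; EnemyDeath schedules the next wave, and Tick prints a debug HUD.
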(event `self.ReceiveTick`
  (params (DeltaSeconds :type "Float (single-precision)"))
  ;[1 0.7647 0] FAKE HUD
  (if (`self.bSpecialWave`)
    (`KismetSystemLibrary.PrintString` (`KismetStringLibrary.Concat_StrStr` "Tempo rimanente per l'ondata speciale : " (`KismetStringLibrary.Conv_IntToString` (`self.SpecialWaveTimeRemaining`))) true true (struct :`G` 0.66 :`B` 1.0 :`A` 1.0) 0.0))
  (`KismetSystemLibrary.PrintString` (`KismetStringLibrary.Concat_StrStr` "Ondata N : " (`KismetStringLibrary.Conv_IntToString` (`self.WaveSpawnedCounter`))) true false (struct :`A` 1.0) 0.0)
  (`KismetSystemLibrary.PrintString` (`KismetStringLibrary.Concat_StrStr` "Nemici totali generati : " (`KismetStringLibrary.Conv_IntToString` (`self.NEnemySpawned`))) true true (struct :`G` 0.66 :`B` 1.0 :`A` 1.0) 0.0)
  (`KismetSystemLibrary.PrintString` (`KismetStringLibrary.Concat_StrStr` "Nemici rimanenti : " (`KismetStringLibrary.Conv_IntToString` (- (`self.NEnemySpawned`) (`self.DeadEnemy`)))) true true (struct :`G` 0.66 :`B` 1.0 :`A` 1.0) 0.0)
  (`KismetSystemLibrary.PrintString` (`KismetStringLibrary.Concat_StrStr` "WaveBetweenParts : " (`KismetStringLibrary.Conv_IntToString` (`self.WaveBetweenTMPSpawn`))) true true (struct :`G` 0.66 :`B` 1.0 :`A` 1.0) 0.0)
  (`KismetSystemLibrary.PrintString` (`KismetStringLibrary.Concat_StrStr` "TimeMachineComponentSpawned : " (`KismetStringLibrary.Conv_BoolToString` (`self.isTimeMachineComponentSpawned`))) true true (struct :`G` 0.66 :`B` 1.0 :`A` 1.0) 0.0))

(event `self.ReceiveBeginPlay`
  (`|ExecutionSequence`
    (:`then_0`
      (`KismetSystemLibrary.Delay` 0.2)
      (bind _outactors (`GameplayStatics.GetAllActorsOfClass` "/Game/Blueprints/SpawnPointTMP_BP.SpawnPointTMP_BP_C"))
      ;[1 1 1] Initial Setup
      (set `self.SpawnPointsTMP` _outactors)
      (bind _returnvalue (`GameplayStatics.GetActorOfClass` "/Game/Blueprints/MainCharacter_BP.MainCharacter_BP_C"))
      (set `self.PlayerRef` _returnvalue)
      (bind _outactors_2 (`GameplayStatics.GetAllActorsOfClass` "/Game/Blueprints/Enemies/EnemySpawner_BP.EnemySpawner_BP_C"))
      (set `self.EnemySpawner` _outactors_2)
      (bind _returnvalue_2 (`GameplayStatics.GetActorOfClass` "/Game/Blueprints/TimeMachine_BP.TimeMachine_BP_C"))
      (set `self.SafeAreaBP` _returnvalue_2)
      (set `self.SpecialWaveTimeRemaining` (`KismetMathLibrary.FTrunc` (`self.SpecialWaveTotalDuration`))))
    (:`then_1`
      (bind _asmy_game_instance (cast `/Game/Blueprints/Core/MyGameInstance` (`GameplayStatics.GetGameInstance`)))
      (set `self.GameInstanceRef` _asmy_game_instance)
      (`self.SpawnWave`))))

(event `SpawnWave`
  ;[1 1 1] LoopStart enemy spawner
  (`self.UpdateWaveCounter`)
  (if (`self.bSpecialWave`)
    (`self.StartSpecialWave`)
    (else
      ;[1 1 1] Spawn loop
      (bind _returnvalue (`KismetSystemLibrary.K2_SetTimer` null "StandardSpawnLoop" 1.2 true))
      (set `self.SpawnerHandle` _returnvalue))))

(event `EnemyDeath`
  (params (EnemyBP :type "/Game/Blueprints/Enemies/EnemyMaster_BP Object Reference"))
  (bind _deadenemy (`self.DeadEnemy`))
  ;[1 1 1] Check if all enemy are dead
  (if (not (`self.bSpecialWave`))
    (`/Engine/EditorBlueprintResources/StandardMacros.IncrementInt` _deadenemy
      (:`  `
        (if (== _deadenemy (`self.NEnemyInWave`))
          (`KismetSystemLibrary.PrintString` "WAVE ENDED!")
          (set `self.NEnemySpawned` 0)
          (set `self.NEnemyInWave` (+ (`self.NEnemyInWave`) (`self.EnemyToAddEachWave`)))
          (set `self.DeadEnemy` 0)
          (`KismetSystemLibrary.K2_SetTimerDelegate` (delegate `SpawnWave`) 5.0))))
    (else
      ;;[1 0 0] DEBUG MA FUNZIONANTE (Special Wave) DA OTTIMIZZARE
      (`/Engine/EditorBlueprintResources/StandardMacros.DecrementInt` (`self.NEnemySpawned`)
        (:`  `
          (bind _outactors (`GameplayStatics.GetAllActorsOfClass` "/Game/Blueprints/Enemies/EnemyMaster_BP.EnemyMaster_BP_C"))
          (`KismetArrayLibrary.Array_RemoveItem` _outactors EnemyBP)
          (if (<= (`KismetArrayLibrary.Array_Length` _outactors) 0)
            (`KismetSystemLibrary.PrintString` "SPECIAL WAVE ENDED!")
            (`KismetSystemLibrary.K2_ClearAndInvalidateTimerHandle` (`self.SpecialWaveCountdownHandle`))
            (set `self.NEnemySpawned` 0)
            (set `self.DeadEnemy` 0)
            (set `self.SpecialWaveTimeRemaining` (`KismetMathLibrary.FTrunc` (`self.SpecialWaveTotalDuration`)))
            (set `self.ActualNormalWaveBetweenSpecial` 0)
            (`KismetSystemLibrary.Delay` 5.0)
            (`self.SpawnWave`)))))))

(event `StartSpecialWave`
  (bind _uiref (`self.UIRef`))
  ;[1 1 1] Special Wave Loops
  (`UserWidget.PlayAnimation` _uiref (`/Game/UI/UI.SpecialWaveAnimation` _uiref) 0.0 3 "Forward" 1.2 false)
  (set `self.NEnemySpawned` 0)
  (bind _returnvalue (`KismetSystemLibrary.K2_SetTimerDelegate` (delegate `SpecialWave`) 1.0 true))
  (set `self.SpecialWaveHandle` _returnvalue)
  (`KismetSystemLibrary.K2_SetTimerDelegate` (delegate `SpecialWaveTimeout`) (`self.SpecialWaveTotalDuration`))
  (bind _returnvalue_2 (`KismetSystemLibrary.K2_SetTimerDelegate` (delegate `SpecialWaveCountdownAndCheckForEnemies`) 1.0 true))
  (set `self.SpecialWaveCountdownHandle` _returnvalue_2))

(event `SpecialWaveCountdownAndCheckForEnemies`
  ;[1 1 1] Special Wave Loops
  (`/Engine/EditorBlueprintResources/StandardMacros.DecrementInt` (`self.SpecialWaveTimeRemaining`)))

(event `SpecialWaveTimeout`
  ;[1 1 1] Special Wave Loops
  (`KismetSystemLibrary.K2_ClearAndInvalidateTimerHandle` (`self.SpecialWaveHandle`)))

(event `SpecialWave`
  ;[1 1 1] Special Wave Loops
  (if (!= (`self.NEnemySpawned`) (`self.SpecialWaveEnemyLimit`))
    (`/Engine/EditorBlueprintResources/StandardMacros.IncrementInt` (`self.NEnemySpawned`)
      (:`  `
        (bind _enemytospawn (`self.GetRandomEnemyToSpawn`))
        (bind _spawnedenemy (`/Game/Blueprints/Enemies/EnemySpawner_BP.SpawnEnemy` (`|GetArrayItem` (`self.EnemySpawner`) (`KismetMathLibrary.RandomIntegerInRange` 0 (- (`KismetArrayLibrary.Array_Length` (`self.EnemySpawner`)) 1))) (`self.SafeAreaBP`) self null _enemytospawn))
        (bind _returnvalue (`KismetArrayLibrary.Array_Add` (`self.EnemySpawned`) _spawnedenemy))
        (set `/Game/Blueprints/Enemies/EnemyMaster_BP.ID` _returnvalue _spawnedenemy)))))

(fn `CheckWaveStatus`
  (if (<= (`self.WaveSpawnedCounter`) 5)
    (set `self.WaveStatus` "NewEnumerator0")
    (return)
    (elif (and (> (`self.WaveSpawnedCounter`) 5) (<= (`self.WaveSpawnedCounter`) 10))
      (set `self.WaveStatus` "NewEnumerator1")
      (return)
      (else
        (if (and (> (`self.WaveSpawnedCounter`) 10) (<= (`self.WaveSpawnedCounter`) 15))
          (set `self.WaveStatus` "NewEnumerator2")
          (else
            (set `self.WaveStatus` "NewEnumerator3")))
        (return)))))

(fn `GetRandomEnemyToSpawn`
  (returns (EnemyToSpawn :type "/Game/Blueprints/Enemies/EnemyMaster_BP Class Reference"))
  (locals (TypesOfEnemies :type "Array of /Game/Blueprints/Enemies/EnemyMaster_BP Class Reference"))
  (switch `/Game/Blueprints/Core/RoundStates` (`self.WaveStatus`)
    (:`NewEnumerator0`
      (return (`|GetArrayItem` (`local.TypesOfEnemies`) 1)))
    (:`NewEnumerator1`
      (bind _enemytospawn (`self.SpawnMidGame`))
      (return _enemytospawn))
    (:`NewEnumerator2`
      (bind _enemytospawn_2 (`self.SpawnLateGame`))
      (return _enemytospawn_2))
    (:`NewEnumerator3`
      (bind _enemytospawn_3 (`self.SpawnUltraLateGame`))
      (return _enemytospawn_3))))

(fn `SpawnLateGame`
  (returns (EnemyToSpawn :type "/Game/Blueprints/Enemies/EnemyMaster_BP Class Reference"))
  (locals (RandomValue :type Integer))
  (bind _output_get (set `local.RandomValue` (`KismetMathLibrary.RandomIntegerInRange` 0 100)))
  (if (<= _output_get 80)
    (return "/Game/Blueprints/Enemies/GroundEnemy/GroundEnemy_BP.GroundEnemy_BP_C")
    (elif (and (> (`local.RandomValue`) 80) (<= (`local.RandomValue`) 84))
      (return "/Game/Blueprints/Enemies/TankEnemy/TankEnemy_BP.TankEnemy_BP_C")
      (elif (and (> (`local.RandomValue`) 84) (<= (`local.RandomValue`) 96))
        (return "/Game/Blueprints/Enemies/GroundEnemy/GroundEnemy_BP.GroundEnemy_BP_C")
        (else
          (return "/Game/Blueprints/Enemies/TankEnemy/TankEnemy_BP.TankEnemy_BP_C"))))))

(fn `SpawnMidGame`
  (returns (EnemyToSpawn :type "/Game/Blueprints/Enemies/EnemyMaster_BP Class Reference"))
  (locals (RandomValue :type Integer))
  (bind _output_get (set `local.RandomValue` (`KismetMathLibrary.RandomIntegerInRange` 0 100)))
  (if (<= _output_get 90)
    (return "/Game/Blueprints/Enemies/GroundEnemy/GroundEnemy_BP.GroundEnemy_BP_C")
    (elif (and (> (`local.RandomValue`) 90) (<= (`local.RandomValue`) 92))
      (return "/Game/Blueprints/Enemies/TankEnemy/TankEnemy_BP.TankEnemy_BP_C")
      (elif (and (> (`local.RandomValue`) 92) (<= (`local.RandomValue`) 96))
        (return "/Game/Blueprints/Enemies/GroundEnemy/GroundEnemy_BP.GroundEnemy_BP_C")
        (else
          (return "/Game/Blueprints/Enemies/TankEnemy/TankEnemy_BP.TankEnemy_BP_C"))))))

(fn `SpawnTimeMachineParts`
  (bind _returnvalue (`|SpawnActorFromClass` "/Game/Blueprints/TimeMachineComponent_BP.TimeMachineComponent_BP_C" (`self.GetTransform` (`KismetArrayLibrary.Array_Random` (`self.SpawnPointsTMP`))) "Undefined" "OverrideRootScale" null self null))
  (set `self.WaveBetweenTMPSpawn` 0)
  (set `self.isTimeMachineComponentSpawned` true)
  (`KismetSystemLibrary.PrintString` (`KismetStringLibrary.Conv_VectorToString` (`self.K2_GetActorLocation` _returnvalue)))
  (return))

(fn `SpawnUltraLateGame`
  (returns (EnemyToSpawn :type "/Game/Blueprints/Enemies/EnemyMaster_BP Class Reference"))
  (locals (RandomValue :type Integer))
  (bind _output_get (set `local.RandomValue` (`KismetMathLibrary.RandomIntegerInRange` 0 100)))
  (if (<= _output_get 65)
    (return "/Game/Blueprints/Enemies/GroundEnemy/GroundEnemy_BP.GroundEnemy_BP_C")
    (elif (and (> (`local.RandomValue`) 65) (<= (`local.RandomValue`) 75))
      (return "/Game/Blueprints/Enemies/TankEnemy/TankEnemy_BP.TankEnemy_BP_C")
      (elif (and (> (`local.RandomValue`) 75) (<= (`local.RandomValue`) 90))
        (return "/Game/Blueprints/Enemies/GroundEnemy/GroundEnemy_BP.GroundEnemy_BP_C")
        (else
          (return "/Game/Blueprints/Enemies/TankEnemy/TankEnemy_BP.TankEnemy_BP_C"))))))

(fn `StandardSpawnLoop`
  (bind _playerref (`self.PlayerRef`))
  (if (!= (`self.NEnemyInWave`) (`self.NEnemySpawned`))
    (`/Engine/EditorBlueprintResources/StandardMacros.IncrementInt` (`self.NEnemySpawned`)
      (:`  `
        (`/Engine/EditorBlueprintResources/StandardMacros.IsValid` _playerref
          (:`Is Valid`
            (bind _enemytospawn (`self.GetRandomEnemyToSpawn`))
            (bind _spawnedenemy (`/Game/Blueprints/Enemies/EnemySpawner_BP.SpawnEnemy` (`|GetArrayItem` (`self.EnemySpawner`) (`KismetMathLibrary.RandomIntegerInRange` 0 (- (`KismetArrayLibrary.Array_Length` (`self.EnemySpawner`)) 1))) _playerref self (`/Game/Blueprints/MainCharacter_BP.CalculatePredictionPoint` _playerref) _enemytospawn))
            (bind _returnvalue (`KismetArrayLibrary.Array_Add` (`self.EnemySpawned`) _spawnedenemy))
            (set `/Game/Blueprints/Enemies/EnemyMaster_BP.ID` _returnvalue _spawnedenemy)))))
    (else
      (`KismetSystemLibrary.K2_ClearAndInvalidateTimerHandle` (`self.SpawnerHandle`)))))

(fn `UpdateWaveCounter`
  (bind _result (`/Engine/EditorBlueprintResources/StandardMacros.IncrementInt` (`self.WaveSpawnedCounter`))
    (:`  `
      (`self.CheckWaveStatus`)
      (set `/Game/Blueprints/Core/MyGameInstance.CompletedStages` _result (`self.GameInstanceRef`))
      (bind _result_2 (`/Engine/EditorBlueprintResources/StandardMacros.IncrementInt` (`self.WaveBetweenTMPSpawn`))
        (:`  `
          (if (and (>= _result_2 (`self.WaveBetweenComponentSpawn`)) (not (`self.isTimeMachineComponentSpawned`)))
            (`self.SpawnTimeMachineParts`))
          (if (== (`self.ActualNormalWaveBetweenSpecial`) (`self.MaxWaveBetweenSpecial`))
            (set `self.ActualNormalWaveBetweenSpecial` 0)
            (set `self.bSpecialWave` true)
            (return)
            (else
              (`/Engine/EditorBlueprintResources/StandardMacros.IncrementInt` (`self.ActualNormalWaveBetweenSpecial`)
                (:`  `
                  (set `self.bSpecialWave` false)
                  (return))))))))))

(fn `UserConstructionScript`)