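; A pickup actor that grants the player a timed stat buff when touched.
; On box overlap with an actor tagged Player, it passes its configured stat, multiplier and duration to MainCharacter_BP's ApplyPowerUp, then destroys itself.
; At BeginPlay it sets its text render label to match the chosen stat: speed, jump, HP regen or shield.
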(event `self.Box.OnComponentBeginOverlap`
  (params (OverlappedComponent :type "PrimitiveComponent Object Reference") (OtherActor :type "Actor Object Reference") (OtherComp :type "PrimitiveComponent Object Reference") (OtherBodyIndex :type Integer) (bFromSweep :type Boolean) (SweepResult :type "HitResult Structure (by ref)"))
  (if (`self.ActorHasTag` OtherActor "Player")
    (`/Game/Blueprints/MainCharacter_BP.ApplyPowerUp` (cast `/Game/Blueprints/MainCharacter_BP` OtherActor :!pure true) (`self.StatToPowerUp`) (`self.Multiplier`) (`self.PowerUpDuration`))
    (`self.K2_DestroyActor`)))

(event `self.ReceiveBeginPlay`
  (switch `/Game/Blueprints/StatsTypes` (`self.StatToPowerUp`)
    (:`NewEnumerator0`
      (`TextRenderComponent.K2_SetText` (`self.TextRender`) "Speed Buff"))
    (:`NewEnumerator1`
      (`TextRenderComponent.K2_SetText` (`self.TextRender`) "Jump Buff"))
    (:`NewEnumerator2`
      (`TextRenderComponent.K2_SetText` (`self.TextRender`) "HP Regen Buff"))
    (:`NewEnumerator5`
      (`TextRenderComponent.K2_SetText` (`self.TextRender`) "Shield"))))

(fn `UserConstructionScript`)