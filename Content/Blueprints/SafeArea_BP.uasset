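; SafeArea_BP is a damageable area with hit points whose loss ends the game.
; On BeginPlay it caches references to the player character and the master enemy spawner.
; HPManagement applies damage only while the spawner's SpecialWave flag is set, updating a text render with the remaining HP.
; When damage would deplete HP, it calls GameOver on the player and destroys itself.
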(event `self.ReceiveBeginPlay`
  (bind _returnvalue (`GameplayStatics.GetActorOfClass` "/Game/Blueprints/MainCharacter_BP.MainCharacter_BP_C"))
  (set `self.PlayerRef` _returnvalue)
  (bind _returnvalue_2 (`GameplayStatics.GetActorOfClass` "/Game/Blueprints/Enemies/EnemySpawner_MasterBP.EnemySpawner_MasterBP_C"))
  (set `self.SpawnerRef` _returnvalue_2))

(event `/Game/Blueprints/Core/HPManagement_Interface.HPManagement`
  (params (DMG :type "Float (single-precision)"))
  (bind _returnvalue (- (`self.HPCurrent`) DMG))
  (if (`/Game/Blueprints/Enemies/EnemySpawner_MasterBP.bSpecialWave` (`self.SpawnerRef`))
    (if (> _returnvalue 0.0)
      (bind _output_get (set `self.HPCurrent` _returnvalue))
      (`TextRenderComponent.K2_SetText` (`self.TextRender`) (`KismetTextLibrary.Conv_DoubleToText` _output_get "HalfToEven"))
      (else
        (`/Game/Blueprints/MainCharacter_BP.GameOver` (`self.PlayerRef`))
        (`self.K2_DestroyActor`)))))

(fn `UserConstructionScript`
  (`TextRenderComponent.K2_SetText` (`self.TextRender`) (`KismetTextLibrary.Conv_DoubleToText` (`self.HPCurrent`) "HalfToEven")))