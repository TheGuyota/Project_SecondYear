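; Master Blueprint for time-travel objects that appear in a different form in each era: past, present or future.
; On BeginPlay it reads ActualEra from MyGameMode, sets its ChildActor class to the matching PastActor, PresentActor or FutureActor, and binds to the game mode's TimeTravelStart event.
; When that event fires, it waits briefly, then swaps the child actor class again to match the current era.
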(event `self.ReceiveBeginPlay`
  (bind _childactor (`self.ChildActor`))
  (bind _asmy_game_mode (cast `/Game/Blueprints/Core/MyGameMode` (`GameplayStatics.GetGameMode`)))
  (bind _output_get (set `self.GameModeRef` _asmy_game_mode))
  (add `/Game/Blueprints/Core/MyGameMode.TimeTravelStart` _output_get (delegate `ChangeEvent`))
  (switch `/Game/Blueprints/TimeTypes` (`/Game/Blueprints/Core/MyGameMode.ActualEra` (`self.GameModeRef`))
    (:`NewEnumerator0`
      (`ChildActorComponent.SetChildActorClass` _childactor (`self.PastActor`)))
    (:`NewEnumerator1`
      (`ChildActorComponent.SetChildActorClass` _childactor (`self.PresentActor`)))
    (:`NewEnumerator2`
      (`ChildActorComponent.SetChildActorClass` _childactor (`self.FutureActor`)))))

(event `ChangeEvent`
  (bind _childactor (`self.ChildActor`))
  (`KismetSystemLibrary.Delay` 1.2)
  (switch `/Game/Blueprints/TimeTypes` (`/Game/Blueprints/Core/MyGameMode.ActualEra` (`self.GameModeRef`))
    (:`NewEnumerator0`
      (`ChildActorComponent.SetChildActorClass` _childactor (`self.PastActor`)))
    (:`NewEnumerator1`
      (`ChildActorComponent.SetChildActorClass` _childactor (`self.PresentActor`)))
    (:`NewEnumerator2`
      (`ChildActorComponent.SetChildActorClass` _childactor (`self.FutureActor`)))))

(fn `UserConstructionScript`)