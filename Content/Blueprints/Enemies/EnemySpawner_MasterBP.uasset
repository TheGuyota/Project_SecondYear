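; Master enemy spawner that runs escalating waves through randomly chosen EnemySpawner_BP actors, with debug prints on Tick as a stand-in HUD.
; Normal waves spawn on a looping timer toward the player's predicted position and grow after all die.
; Periodic special waves target the SafeArea, refill to a live cap until timeout, and end when a death leaves no enemies.
; WaveManagement behaviour switching is unfinished and never started.
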(event `self.ReceiveTick`
  (params (DeltaSeconds :type "Float (single-precision)"))
  ;[1 0.7647 0] FAKE HUD
  (if (`self.bSpecialWave`)
    (`KismetSystemLibrary.PrintString` (`KismetStringLibrary.Concat_StrStr` "Tempo rimanente per l'ondata speciale : " (`KismetStringLibrary.Conv_IntToString` (`self.SpecialWaveTimeRemaining`))) true true (struct :`G` 0.66 :`B` 1.0 :`A` 1.0) 0.0))
  (`KismetSystemLibrary.PrintString` (`KismetStringLibrary.Concat_StrStr` "Ondata N : " (`KismetStringLibrary.Conv_IntToString` (`self.WaveSpawnedCounter`))) true false (struct :`A` 1.0) 0.0)
  (`KismetSystemLibrary.PrintString` (`KismetStringLibrary.Concat_StrStr` "Nemici totali generati : " (`KismetStringLibrary.Conv_IntToString` (`self.NEnemySpawned`))) true true (struct :`G` 0.66 :`B` 1.0 :`A` 1.0) 0.0)
  (`KismetSystemLibrary.PrintString` (`KismetStringLibrary.Concat_StrStr` "Nemici rimanenti : " (`KismetStringLibrary.Conv_IntToString` (- (`self.NEnemySpawned`) (`self.DeadEnemy`)))) true true (struct :`G` 0.66 :`B` 1.0 :`A` 1.0) 0.0))

(event `self.ReceiveBeginPlay`
  (`|ExecutionSequence`
    (:`then_0`
      ;[1 1 1] Initial Setup
      (`KismetSystemLibrary.Delay` 0.2)
      (bind _returnvalue (`GameplayStatics.GetActorOfClass` "/Game/Blueprints/MainCharacter_BP.MainCharacter_BP_C"))
      (set `self.PlayerRef` _returnvalue)
      (bind _outactors (`GameplayStatics.GetAllActorsOfClass` "/Game/Blueprints/Enemies/EnemySpawner_BP.EnemySpawner_BP_C"))
      (set `self.EnemySpawner` _outactors)
      (bind _returnvalue_2 (`GameplayStatics.GetActorOfClass` "/Game/Blueprints/SafeArea_BP.SafeArea_BP_C"))
      (set `self.SafeAreaBP` _returnvalue_2)
      (set `self.SpecialWaveTimeRemaining` (`KismetMathLibrary.FTrunc` (`self.SpecialWaveTotalDuration`)))
      (`self.SpawnWave`))))

(event `SpawnWave`
  ;[1 1 1] LoopStart enemy spawner
  (`self.UpdateWaveCounter`)
  (if (`self.bSpecialWave`)
    (`self.StartSpecialWave`)
    (else
      ;[1 1 1] Spawn loop
      (bind _returnvalue (`KismetSystemLibrary.K2_SetTimer` null "StandardSpawnLoop" 1.2 true))
      (set `self.SpawnerHandle` _returnvalue))))

(event `EnemyDeath`
  (params (EnemyBP :type "/Game/Blueprints/Enemies/Enemy_BP Object Reference"))
  (bind _deadenemy (`self.DeadEnemy`))
  ;[1 1 1] Check if all enemy are dead
  (if (not (`self.bSpecialWave`))
    (`/Engine/EditorBlueprintResources/StandardMacros.IncrementInt` _deadenemy
      (:`  `
        (if (== _deadenemy (`self.NEnemyInWave`))
          (`KismetSystemLibrary.PrintString` "WAVE ENDED!")
          (set `self.NEnemySpawned` 0)
          (set `self.NEnemyInWave` (+ (`self.NEnemyInWave`) (`self.EnemyToAddEachWave`)))
          (set `self.DeadEnemy` 0)
          (`KismetSystemLibrary.K2_SetTimerDelegate` (delegate `SpawnWave`) 5.0))))
    (else
      ;;[1 0 0] DEBUG MA FUNZIONANTE (Special Wave) DA OTTIMIZZARE
      (`/Engine/EditorBlueprintResources/StandardMacros.DecrementInt` (`self.NEnemySpawned`)
        (:`  `
          (bind _outactors (`GameplayStatics.GetAllActorsOfClass` "/Game/Blueprints/Enemies/Enemy_BP.Enemy_BP_C"))
          (`KismetArrayLibrary.Array_RemoveItem` _outactors EnemyBP)
          (if (<= (`KismetArrayLibrary.Array_Length` _outactors) 0)
            (`KismetSystemLibrary.PrintString` "SPECIAL WAVE ENDED!")
            (`KismetSystemLibrary.K2_ClearAndInvalidateTimerHandle` (`self.SpecialWaveCountdownHandle`))
            (set `self.NEnemySpawned` 0)
            (set `self.DeadEnemy` 0)
            (set `self.SpecialWaveTimeRemaining` (`KismetMathLibrary.FTrunc` (`self.SpecialWaveTotalDuration`)))
            (set `self.ActualNormalWaveBetweenSpecial` 0)
            (`KismetSystemLibrary.Delay` 5.0)
            (`self.SpawnWave`)))))))

(event `StartSpecialWave`
  ;[1 1 1] Special Wave Loops
  (`KismetSystemLibrary.PrintString` "SpecialWave")
  (set `self.NEnemySpawned` 0)
  (bind _returnvalue (`KismetSystemLibrary.K2_SetTimerDelegate` (delegate `SpecialWave`) 1.0 true))
  (set `self.SpecialWaveHandle` _returnvalue)
  (`KismetSystemLibrary.K2_SetTimerDelegate` (delegate `SpecialWaveTimeout`) (`self.SpecialWaveTotalDuration`))
  (bind _returnvalue_2 (`KismetSystemLibrary.K2_SetTimerDelegate` (delegate `SpecialWaveCountdownAndCheckForEnemies`) 1.0 true))
  (set `self.SpecialWaveCountdownHandle` _returnvalue_2))

(event `WaveManagement`
  ;[1 0 0] DA IMPLEMENTARE
  (switch `/Game/Blueprints/Enemies/GenericEnemiesBehaviourType` (`self.WaveBehaviour`)
    (:`NewEnumerator0`
      (if (< (`KismetArrayLibrary.Array_Length` (`self.EnemySpawned`)) 10)
        (`self.<10BehaviourSet`)
        (else
          (`self.>10BehaviourSet`))))
    (:`NewEnumerator1`
      (`self.StandardBehaviourSet` :!label _label))
    (:`NewEnumerator2`
      (goto _label))))

(event `SpecialWave`
  ;[1 1 1] Special Wave Loops
  (if (!= (`self.NEnemySpawned`) (`self.SpecialWaveEnemyLimit`))
    (`/Engine/EditorBlueprintResources/StandardMacros.IncrementInt` (`self.NEnemySpawned`)
      (:`  `
        (bind _spawnedenemy (`/Game/Blueprints/Enemies/EnemySpawner_BP.SpawnEnemy` (`|GetArrayItem` (`self.EnemySpawner`) (`KismetMathLibrary.RandomIntegerInRange` 0 (- (`KismetArrayLibrary.Array_Length` (`self.EnemySpawner`)) 1))) (`self.SafeAreaBP`) self null))
        (bind _returnvalue (`KismetArrayLibrary.Array_Add` (`self.EnemySpawned`) _spawnedenemy))
        (set `/Game/Blueprints/Enemies/Enemy_BP.ID` _returnvalue _spawnedenemy)))))

(event `SpecialWaveTimeout`
  ;[1 1 1] Special Wave Loops
  (`KismetSystemLibrary.K2_ClearAndInvalidateTimerHandle` (`self.SpecialWaveHandle`)))

(event `SpecialWaveCountdownAndCheckForEnemies`
  ;[1 1 1] Special Wave Loops
  (`/Engine/EditorBlueprintResources/StandardMacros.DecrementInt` (`self.SpecialWaveTimeRemaining`)))

(fn `<10BehaviourSet`
  (set `self.WaveBehaviour` "NewEnumerator1")
  (for (_ _array_index) (`self.EnemySpawned`)
    (if (== (mod (mod _array_index 3) 2) 0)
      _)))

(fn `>10BehaviourSet`
  (set `self.WaveBehaviour` "NewEnumerator2"))

(fn `StandardBehaviourSet`
  (set `self.WaveBehaviour` "NewEnumerator0")
  (for _array_element (`self.EnemySpawned`)
    (set `/Game/Blueprints/Enemies/Enemy_BP.PredictionTarget` (`/Game/Blueprints/MainCharacter_BP.CalculatePredictionPoint` (`self.PlayerRef`)) _array_element))
  (return))

(fn `StandardSpawnLoop`
  (bind _playerref (`self.PlayerRef`))
  (if (!= (`self.NEnemyInWave`) (`self.NEnemySpawned`))
    (`/Engine/EditorBlueprintResources/StandardMacros.IncrementInt` (`self.NEnemySpawned`)
      (:`  `
        (bind _spawnedenemy (`/Game/Blueprints/Enemies/EnemySpawner_BP.SpawnEnemy` (`|GetArrayItem` (`self.EnemySpawner`) (`KismetMathLibrary.RandomIntegerInRange` 0 (- (`KismetArrayLibrary.Array_Length` (`self.EnemySpawner`)) 1))) _playerref self (`/Game/Blueprints/MainCharacter_BP.CalculatePredictionPoint` _playerref)))
        (bind _returnvalue (`KismetArrayLibrary.Array_Add` (`self.EnemySpawned`) _spawnedenemy))
        (set `/Game/Blueprints/Enemies/Enemy_BP.ID` _returnvalue _spawnedenemy)))
    (else
      (`KismetSystemLibrary.K2_ClearAndInvalidateTimerHandle` (`self.SpawnerHandle`)))))

(fn `UpdateWaveCounter`
  (`/Engine/EditorBlueprintResources/StandardMacros.IncrementInt` (`self.WaveSpawnedCounter`)
    (:`  `
      (if (== (`self.ActualNormalWaveBetweenSpecial`) (`self.MaxWaveBetweenSpecial`))
        (set `self.ActualNormalWaveBetweenSpecial` 0)
        (set `self.bSpecialWave` true)
        (return)
        (else
          (`/Engine/EditorBlueprintResources/StandardMacros.IncrementInt` (`self.ActualNormalWaveBetweenSpecial`)
            (:`  `
              (set `self.bSpecialWave` false)
              (return))))))))

(fn `UserConstructionScript`)