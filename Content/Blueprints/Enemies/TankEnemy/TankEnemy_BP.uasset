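; Tank enemy that chases and punches its target, retargeting to whoever damages it and taking half damage on its front collision.
; AI MoveTo leads into a punch montage, then resumes the chase; AttackDamage sphere-traces at the fist and sends damage through HPManagement_Interface.
; Health and level show on text components.
; At zero HP it reports to the master spawner, calling DestroyEnemy only if the target is the main character.
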(event `self.ReceivePointDamage`
  (params (Damage :type "Float (single-precision)") (DamageType :type "DamageType Object Reference") (HitLocation :type "Vector Structure") (HitNormal :type "Vector Structure") (HitComponent :type "PrimitiveComponent Object Reference") (BoneName :type Name) (ShotFromDirection :type "Vector Structure") (InstigatedBy :type "Controller Object Reference") (DamageCauser :type "Actor Object Reference") (HitInfo :type "HitResult Structure (by ref)"))
  ;[1 1 1] Apply Point Damage
  (`KismetSystemLibrary.PrintString` (`KismetSystemLibrary.GetDisplayName` HitComponent))
  (if (!= DamageCauser (`self.TargetRef`))
    (set `self.TargetRef` DamageCauser)
    (`self.HPManagement` Damage HitComponent)
    (else
      (`self.HPManagement` Damage HitComponent))))

(event `self.ReceiveBeginPlay`
  ;[1 1 1] BeginPlay
  (`parent.ReceiveBeginPlay`)
  (`|ExecutionSequence`
    (:`then_0`
      (`self.ChasePlayer`))
    (:`then_1`
      (bind _output_get (set `self.HPCurrent` (`self.HPMax`)))
      (`TextRenderComponent.K2_SetText` (`self.TextRender`) (`KismetTextLibrary.Conv_DoubleToText` _output_get "HalfToEven")))))

(event `self.ReceiveTick`
  (params (DeltaSeconds :type "Float (single-precision)"))
  (`TextRenderComponent.K2_SetText` (`self.Elv`) (`KismetTextLibrary.Conv_IntToText` (`self.EnemyLevel`)))
  (`TextRenderComponent.K2_SetText` (`self.MaxHP`) (`KismetTextLibrary.Conv_DoubleToText` (`self.HPMax`) "HalfToEven")))

(event `AttackPlayer`
  ;[1 1 1] AttackSequence
  (`|PlayMontage` (`self.Mesh`) "/Game/Animations/TankEnemy/TankEnemyPunch_AnimMontage.TankEnemyPunch_AnimMontage"
    (:`OnCompleted`
      (`KismetSystemLibrary.Delay` 0.3)
      (`self.ChasePlayer`))))

(event `self.HPManagement`
  (params (DMG :type "Float (single-precision)") (HitComponent :type "PrimitiveComponent Object Reference"))
  ;[1 1 1] INTERFACE
  (`self.ApplyScaledDamage` (select `bool` (== HitComponent (`self.FrontCollision`)) :`false` DMG :`true` (/ DMG 2.0))))

(event `ChasePlayer`
  (bind _targetref (`self.TargetRef`))
  (bind (_returnvalue_roll _returnvalue_pitch _returnvalue_yaw) (`KismetMathLibrary.BreakRotator` (`KismetMathLibrary.FindLookAtRotation` (`self.K2_GetActorLocation`) (`self.K2_GetActorLocation` _targetref))))
  ;[1 1 1] Movement
  (`/Engine/EditorBlueprintResources/StandardMacros.IsValid` (`self.TargetRef`)
    (:`Is Valid`
      (`AIController.K2_SetFocus` (`AIBlueprintHelperLibrary.GetAIController` self) null)
      (`|AIMoveTo` self (0.0 0.0 0.0) (`self.TargetRef`) 100.0
        (:`OnSuccess`
          (`self.AttackPlayer`)
          (if (== _targetref "/Game/Blueprints/MainCharacter_BP.MainCharacter_BP")
            (`AIController.K2_ClearFocus` (`AIBlueprintHelperLibrary.GetAIController` self))
            (else
              (`/Engine/EditorBlueprintResources/StandardMacros.IsValid` _targetref
                (:`Is Valid`
                  (`self.K2_SetActorRotation` (`KismetMathLibrary.MakeRotator` 0.0 0.0 _returnvalue_yaw)))))))))))

(event `ApplyScaledDamage`
  (params (EffectiveDamage :type "Float (double-precision)"))
  (bind _masterspawnerref (`self.MasterSpawnerRef`))
  (bind _returnvalue (- (`self.HPCurrent`) EffectiveDamage))
  ;[1 1 1] Apply the right damage
  (if (> _returnvalue 0.0)
    (bind _output_get (set `self.HPCurrent` _returnvalue))
    (`TextRenderComponent.K2_SetText` (`self.TextRender`) (`KismetTextLibrary.Conv_DoubleToText` _output_get "HalfToEven"))
    (else
      (`/Game/Blueprints/SpawnManager_MasterBP.EnemyDeath` _masterspawnerref self)
      (`KismetArrayLibrary.Array_Remove` (`/Game/Blueprints/SpawnManager_MasterBP.EnemySpawned` _masterspawnerref) (`self.ID`))
      (bind _asmain_character_bp (cast `/Game/Blueprints/MainCharacter_BP` (`self.TargetRef`)))
      (`self.Destroy Enemy` _asmain_character_bp))))

(fn `AttackDamage`
  (bind _returnvalue (`SceneComponent.K2_GetComponentLocation` (`self.Punch`)))
  (bind _outhits (`KismetSystemLibrary.SphereTraceMulti` :`Start` _returnvalue :`End` _returnvalue :`Radius` 80.0 :`TraceChannel` "TraceTypeQuery6" :`DrawTime` 2.0))
  (for _array_element _outhits
    (bind (_bblockinghit _binitialoverlap _time _distance _location _impactpoint _normal _impactnormal _physmat _hitactor) (`GameplayStatics.BreakHitResult` _array_element))
    (if (`KismetSystemLibrary.DoesImplementInterface` _hitactor "/Game/Blueprints/Core/HPManagement_Interface.HPManagement_Interface_C")
      (message `/Game/Blueprints/Core/HPManagement_Interface.HPManagement` _hitactor (`self.DMG`) null)))
  (return))

(fn `UserConstructionScript`)