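; Ground enemy that takes damage, attacks nearby actors and can drop a power-up on death.
; Point damage can retarget its AI controller to the attacker and quadruples headshots before updating health and the text display.
; Death notifies the master spawner and spawns any drop pre-rolled at BeginPlay, with the BonusToken branch disabled.
; Attacks use a sphere trace, applying damage through the HP management interface.
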(event `self.ReceiveBeginPlay`
  (`|ExecutionSequence`
    (:`then_0`
      ;[1 1 1] Set Droprate
      (set `self.DropRate` (`KismetMathLibrary.RandomFloatInRange` 0.0 100.0))
      (`self.SetupDropRate`))))

(event `self.ReceivePointDamage`
  (params (Damage :type "Float (single-precision)") (DamageType :type "DamageType Object Reference") (HitLocation :type "Vector Structure") (HitNormal :type "Vector Structure") (HitComponent :type "PrimitiveComponent Object Reference") (BoneName :type Name) (ShotFromDirection :type "Vector Structure") (InstigatedBy :type "Controller Object Reference") (DamageCauser :type "Actor Object Reference") (HitInfo :type "HitResult Structure (by ref)"))
  ;[1 1 1] TakeDamage
  (if (or (!= DamageCauser (`self.TargetRef`)) (not (`KismetSystemLibrary.IsValid` (`self.PredictionTarget`))))
    (set `self.TargetRef` DamageCauser)
    (`/Game/Blueprints/Enemies/GroundEnemy/Enemy_AIController.UpdateTarget` (cast `/Game/Blueprints/Enemies/GroundEnemy/Enemy_AIController` (`self.GetController`) :!pure true)))
  (if (== BoneName "head")
    (`self.HPManagement` (* 4 Damage))
    (else
      (`self.HPManagement` Damage))))

(event `self.HPManagement`
  (params (DMG :type "Float (single-precision)") (HitComponent :type "PrimitiveComponent Object Reference"))
  (bind _masterspawnerref (`self.MasterSpawnerRef`))
  (bind _returnvalue (- (`self.HPCurrent`) DMG))
  ;[1 1 1] HpManagement (Interface)
  (if (> _returnvalue 0.0)
    (bind _output_get (set `self.HPCurrent` _returnvalue))
    (`TextRenderComponent.K2_SetText` (`self.TextRender`) (`KismetTextLibrary.Conv_DoubleToText` _output_get "HalfToEven"))
    (else
      (`/Game/Blueprints/Enemies/EnemySpawner_MasterBP.EnemyDeath` _masterspawnerref self)
      (`KismetArrayLibrary.Array_Remove` (`/Game/Blueprints/Enemies/EnemySpawner_MasterBP.EnemySpawned` _masterspawnerref) (`self.ID`))
      (`self.SpawnDrop`)
      (`self.K2_DestroyActor`))))

(fn `AttackDamageFunction`
  (bind _returnvalue (`SceneComponent.K2_GetComponentLocation` (`self.Scene`)))
  (bind _outhits (`KismetSystemLibrary.SphereTraceMulti` :`Start` _returnvalue :`End` _returnvalue :`Radius` 150.0 :`TraceChannel` "TraceTypeQuery6" :`DrawDebugType` "ForDuration" :`DrawTime` 2.0))
  (for _array_element _outhits
    (bind (_bblockinghit _binitialoverlap _time _distance _location _impactpoint _normal _impactnormal _physmat _hitactor) (`GameplayStatics.BreakHitResult` _array_element))
    (if (`KismetSystemLibrary.DoesImplementInterface` _hitactor "/Game/Blueprints/Core/HPManagement_Interface.HPManagement_Interface_C")
      (message `/Game/Blueprints/Core/HPManagement_Interface.HPManagement` _hitactor (`self.DMG`) null)))
  (return))

(fn `SetupDropRate`
  (if (<= (`self.DropRate`) 90.0)
    (return)
    (elif (and (> (`self.DropRate`) 90.0) (<= (`self.DropRate`) 94.25))
      (set `self.DropToSpawn` "/Game/Blueprints/PowerUp/PiedeLesto_BP.PiedeLesto_BP_C")
      (return)
      (elif (and (> (`self.DropRate`) 94.25) (<= (`self.DropRate`) 98.5))
        (set `self.DropToSpawn` "/Game/Blueprints/PowerUp/BalzoDelConiglio_BP.BalzoDelConiglio_BP_C")
        (return)
        (elif (and (> (`self.DropRate`) 98.5) (<= (`self.DropRate`) 99.5))
          (set `self.DropToSpawn` "/Game/Blueprints/PowerUp/Berserk_BP.Berserk_BP_C")
          (return)
          (else
            ;[1 1 1] BonusToken
            (if (and (> (`self.DropRate`) 99.5) false)
              (set `self.DropToSpawn` "/Game/Blueprints/PowerUp/BonusToken_BP.BonusToken_BP_C")
              (return)
              (else
                (return)))))))))

(fn `SpawnDrop`
  (bind _returnvalue (`KismetMathLibrary.Conv_IntToDouble` (`KismetMathLibrary.RandomIntegerInRange` 4 8)))
  (if (> (`self.DropRate`) 90.0)
    (`|SpawnActorFromClass` (`self.DropToSpawn`) (`self.GetTransform`) "AlwaysSpawn" "OverrideRootScale" null _returnvalue false (+ _returnvalue 5.0) null)
    (return)))

(fn `UserConstructionScript`
  (set `self.HPCurrent` (`self.HPMax`)))