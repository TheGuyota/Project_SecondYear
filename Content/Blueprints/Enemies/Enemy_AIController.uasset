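; AI controller for Enemy_BP pawns that starts their behavior tree and flags attacks.
; On possess, it waits briefly, caches the pawn as an Enemy_BP reference, runs Enemy_BT and copies the pawn's TargetRef into the blackboard.
; An Attack function sets IsAttacking on the cached enemy, leaving the attack itself to be handled outside the controller.
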(event `self.ReceivePossess`
  (params (PossessedPawn :type "Pawn Object Reference"))
  (bind _asenemy_bp (cast `/Game/Blueprints/Enemies/Enemy_BP` PossessedPawn :!pure true))
  (`KismetSystemLibrary.Delay` 0.2)
  (set `self.EnemySelfRef` _asenemy_bp)
  (`self.RunBehaviorTree` "/Game/Blueprints/Enemies/Enemy_BT.Enemy_BT")
  (`BlackboardComponent.SetValueAsObject` (`self.Blackboard`) "TargetRef" (`/Game/Blueprints/Enemies/Enemy_BP.TargetRef` _asenemy_bp)))

(fn `Attack`
  (set `/Game/Blueprints/Enemies/Enemy_BP.isAttacking` true (`self.EnemySelfRef`))
  (return))

(fn `UserConstructionScript`)