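; Behavior tree task that makes an enemy chase the actor stored in the TargetRef blackboard key.
; It starts AI MoveTo toward the target and finishes with success or failure from the move result.
; Alongside the move, a looping timer polls distance and, within a short range, stops the Enemy_BP's movement and finishes successfully.
; The graph never clears that timer.
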(event `self.ReceiveExecuteAI`
  (params (OwnerController :type "AIController Object Reference") (ControlledPawn :type "Pawn Object Reference"))
  (`|AIMoveTo` ControlledPawn (0.0 0.0 0.0) (`BTFunctionLibrary.GetBlackboardValueAsActor` (`self.TargetRef`))
    (:`then`
      (`KismetSystemLibrary.K2_SetTimerDelegate` (delegate `CheckDistanceOfTarget`) 0.1 true))
    (:`OnSuccess`
      (`self.FinishExecute` true))
    (:`OnFail`
      (`self.FinishExecute` false))))

(event `CheckDistanceOfTarget`
  (`/Engine/EditorBlueprintResources/StandardMacros.IsValid` (`BTFunctionLibrary.GetBlackboardValueAsActor` (`self.TargetRef`))
    (:`Is Valid`
      (if (< (`KismetMathLibrary.Vector_Distance` (`Actor.K2_GetActorLocation` (stale `self.ReceiveExecuteAI` ControlledPawn)) (`Actor.K2_GetActorLocation` (`BTFunctionLibrary.GetBlackboardValueAsActor` (`self.TargetRef`)))) 200.0)
        (`MovementComponent.StopMovementImmediately` (`Character.CharacterMovement` (cast `/Game/Blueprints/Enemies/Enemy_BP` (`BTFunctionLibrary.GetBlackboardValueAsActor` (`self.SelfRef`)) :!pure true)))
        (`self.FinishExecute` true)))))