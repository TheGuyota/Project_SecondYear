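; Behavior Tree task that moves an Enemy_BP pawn toward its PredictionTarget actor.
; It gets the enemy from the SelfRef blackboard key and starts AIMoveTo, finishing with the move's result, or successfully if no valid target exists.
; Once movement starts, a looping timer checks distance, setting IsInAttackRange and ending the task early when the target is close, or just ending it if the target becomes invalid.
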(event `self.ReceiveExecuteAI`
  (params (OwnerController :type "AIController Object Reference") (ControlledPawn :type "Pawn Object Reference"))
  (bind _asenemy_bp (cast `/Game/Blueprints/Enemies/Enemy_BP` (`BTFunctionLibrary.GetBlackboardValueAsActor` (`self.SelfRef`))))
  (set `self.EnemyRef` _asenemy_bp)
  (bind _predictiontarget (`/Game/Blueprints/Enemies/Enemy_BP.PredictionTarget` _asenemy_bp))
  (`/Engine/EditorBlueprintResources/StandardMacros.IsValid` _predictiontarget
    (:`Is Valid`
      (`|AIMoveTo` ControlledPawn (0.0 0.0 0.0) _predictiontarget 10.0
        (:`then`
          (`KismetSystemLibrary.K2_SetTimerDelegate` (delegate `CheckDistance`) 0.1 true))
        (:`OnSuccess`
          (`self.FinishExecute` true))
        (:`OnFail`
          (`self.FinishExecute` false))))
    (:`Is Not Valid`
      (`self.FinishExecute` true))))

(event `CheckDistance`
  (bind _enemyref (`self.EnemyRef`))
  (bind _predictiontarget (`/Game/Blueprints/Enemies/Enemy_BP.PredictionTarget` _enemyref))
  (`/Engine/EditorBlueprintResources/StandardMacros.IsValid` _predictiontarget
    (:`Is Valid`
      (if (< (`KismetMathLibrary.Vector_Distance` (`Actor.K2_GetActorLocation` _enemyref) (`Actor.K2_GetActorLocation` _predictiontarget)) 450.0)
        (`BTFunctionLibrary.SetBlackboardValueAsBool` (`self.isInAttackRange`) true)
        (`self.FinishExecute` true)))
    (:`Is Not Valid`
      (`self.FinishExecute` true))))