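; Enemy actor that takes point damage, with quadrupled headshots, and may leave a timed power-up when killed.
; A random roll at BeginPlay preselects the drop and shows a debug label; the bonus-token branch is disabled.
; HPManagement, an interface event, subtracts health and on death notifies the master spawner, spawns any TestBuff_BP drop and destroys the actor.
; ResetCollision restores the Enemy collision profile after a delay.
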(event `self.ReceiveBeginPlay`
  (`|ExecutionSequence`
    (:`then_0`
      ;[1 1 1] Set Droprate
      (set `self.DropRate` (`KismetMathLibrary.RandomFloatInRange` 0.0 100.0))
      (`self.SetupDropRate`))))

(event `self.ReceivePointDamage`
  (params (Damage :type "Float (single-precision)") (DamageType :type "DamageType Object Reference") (HitLocation :type "Vector Structure") (HitNormal :type "Vector Structure") (HitComponent :type "PrimitiveComponent Object Reference") (BoneName :type Name) (ShotFromDirection :type "Vector Structure") (InstigatedBy :type "Controller Object Reference") (DamageCauser :type "Actor Object Reference") (HitInfo :type "HitResult Structure (by ref)"))
  ;[1 1 1] TakeDamage
  (if (== BoneName "head")
    (`self.HPManagement` (* 4 Damage))
    (else
      (`self.HPManagement` Damage))))

(event `ResetCollision`
  (`KismetSystemLibrary.Delay` 2.0)
  (`PrimitiveComponent.SetCollisionProfileName` (`self.CapsuleComponent`) "Enemy" true))

(event `self.HPManagement`
  (params (DMG :type "Float (single-precision)"))
  (bind _returnvalue (- (`self.HPCurrent`) DMG))
  ;[1 1 1] HpManagement (Interface)
  (if (> _returnvalue 0.0)
    (set `self.HPCurrent` _returnvalue)
    (else
      (`/Game/Blueprints/Enemies/EnemySpawner_MasterBP.EnemyDeath` (`self.MasterSpawnerRef`))
      (`self.SpawnDrop`)
      (`self.K2_DestroyActor`))))

(fn `SetupDropRate`
  (bind _debug_dropornot (`self.DEBUG-DropOrNot`))
  (if (<= (`self.DropRate`) 90.0)
    ;[1 0 0] Temp DEBUG
    (`TextRenderComponent.K2_SetText` _debug_dropornot "NO DROP")
    (return)
    (else
      (`TextRenderComponent.K2_SetText` _debug_dropornot "DROP")
      (if (and (> (`self.DropRate`) 90.0) (<= (`self.DropRate`) 94.25))
        (set `self.DropToSpawn` "NewEnumerator0")
        (return)
        (elif (and (> (`self.DropRate`) 94.25) (<= (`self.DropRate`) 98.5))
          (set `self.DropToSpawn` "NewEnumerator1")
          (return)
          (elif (and (> (`self.DropRate`) 98.5) (<= (`self.DropRate`) 99.5))
            (set `self.DropToSpawn` "NewEnumerator6")
            (return)
            (else
              ;[1 1 1] BonusToken
              (if (and (> (`self.DropRate`) 99.5) false)
                (`KismetSystemLibrary.PrintString` "BonusToken!")
                (return)
                (else
                  (return))))))))))

(fn `SpawnDrop`
  (if (> (`self.DropRate`) 90.0)
    (`|SpawnActorFromClass` "/Game/Blueprints/TestBuff_BP.TestBuff_BP_C" (`self.GetTransform`) "AlwaysSpawn" "OverrideRootScale" null (`self.DropToSpawn`) 2.0 5.0 false 15.0 null)
    (return)))

(fn `UserConstructionScript`
  (set `self.HPCurrent` (`self.HPMax`)))