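; Master enemy Blueprint that scales difficulty, health and XP reward as the game progresses.
; On spawn and each game mode time-travel event, it increments a time counter and combines it with completed stages to compute level and XP.
; Max HP compounds for each level above LastLvlValue.
; DestroyEnemy awards XP to the given player before destroying the actor, and ResetCollision restores the Enemy capsule profile after a delay.
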(event `ResetCollision`
  (`KismetSystemLibrary.Delay` 2.0)
  (`PrimitiveComponent.SetCollisionProfileName` (`self.CapsuleComponent`) "Enemy" true))

(event `self.ReceiveBeginPlay`
  (bind _asmy_game_mode (cast `/Game/Blueprints/Core/MyGameMode` (`GameplayStatics.GetGameMode`)))
  (add `/Game/Blueprints/Core/MyGameMode.TimeTravelStart` _asmy_game_mode (delegate `UpdateEnemyLevel`))
  (bind _asmy_game_instance (cast `/Game/Blueprints/Core/MyGameInstance` (`GameplayStatics.GetGameInstance`)))
  (set `self.GameInstanceRef` _asmy_game_instance)
  (`self.UpdateEnemyLevel`))

(event `UpdateEnemyLevel`
  (`/Engine/EditorBlueprintResources/StandardMacros.IncrementInt` (`self.TimeInt`)
    (:`  `
      (bind _output_get (set `self.StageFactor` (`KismetMathLibrary.MultiplyMultiply_FloatFloat` 1.05 (`KismetMathLibrary.Conv_IntToDouble` (`/Game/Blueprints/Core/MyGameInstance.CompletedStages` (`self.GameInstanceRef`))))))
      (bind _returnvalue (* (+ 1.2 (* (`self.TimeInt`) 0.05)) _output_get))
      ;[1 1 1] Livello Nemico
      (set `self.EnemyLevel` (`KismetMathLibrary.FTrunc` (/ (+ 1.0 (- _returnvalue 1.2)) 0.3)))
      ;[1 1 1] Aggiorno il valore della vita massima
      (`self.UpdateHPMax`)
      ;[1 1 1] UpdateXPReward
      (set `self.XPReward` (* _returnvalue (`KismetMathLibrary.Conv_IntToDouble` (`self.EnemyValue`)))))))

(fn `Destroy Enemy`
  (params (PlayerRef :type "/Game/Blueprints/MainCharacter_BP Object Reference"))
  (`/Game/Blueprints/MainCharacter_BP.EXPSystem` PlayerRef (`self.XPReward`))
  (`self.K2_DestroyActor`))

(fn `UpdateHPMax`
  (locals (lvlsToAdd :type Integer))
  (bind _output_get (set `local.lvlsToAdd` (- (`self.EnemyLevel`) (`self.LastLvlValue`))))
  (for _ (range 1 (+ _output_get 1))
    (set `self.HPMax` (+ (`self.HPMax`) (* (`self.HPMax`) 0.1))))
  (return))

(fn `UserConstructionScript`)