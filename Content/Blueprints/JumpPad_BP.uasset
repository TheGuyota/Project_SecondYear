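; Jump pad that launches an overlapping player-tagged MainCharacter in a selectable direction.
; The construction script orients an arrow to front, right, left, back or up, then precomputes the impulse from its forward vector, force and vertical offset.
; On overlap it stops movement and applies that impulse as a velocity change.
; A one-second timer then checks the stored character reference, which is cleared when the player leaves.
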(event `Redo Jump`
  (bind _charactermovement (`Character.CharacterMovement` (cast `/Game/Blueprints/MainCharacter_BP` (stale `self.Box.OnComponentBeginOverlap` OtherActor) :!pure true)))
  (`MovementComponent.StopMovementImmediately` _charactermovement :!label _label)
  (`CharacterMovementComponent.AddImpulse` _charactermovement (`self.DefinitiveImpulse`) true)
  (`KismetSystemLibrary.K2_SetTimerDelegate` (delegate `CheckFunc`) 1.0))

(event `self.Box.OnComponentBeginOverlap`
  (params (OverlappedComponent :type "PrimitiveComponent Object Reference") (OtherActor :type "Actor Object Reference") (OtherComp :type "PrimitiveComponent Object Reference") (OtherBodyIndex :type Integer) (bFromSweep :type Boolean) (SweepResult :type "HitResult Structure (by ref)"))
  (if (`self.ActorHasTag` OtherActor "Player")
    (set `self.MainCharacterRef` (cast `/Game/Blueprints/MainCharacter_BP` OtherActor :!pure true))
    (goto _label)))

(event `CheckFunc`
  (`/Engine/EditorBlueprintResources/StandardMacros.IsValid` (`self.MainCharacterRef`)
    (:`Is Valid`
      (`self.CheckFunc`))))

(event `self.Box.OnComponentEndOverlap`
  (params (OverlappedComponent :type "PrimitiveComponent Object Reference") (OtherActor :type "Actor Object Reference") (OtherComp :type "PrimitiveComponent Object Reference") (OtherBodyIndex :type Integer))
  (if (`self.ActorHasTag` OtherActor "Player")
    (set `self.MainCharacterRef` null)))

(fn `UserConstructionScript`
  (bind (_returnvalue_x _returnvalue_y _returnvalue_z) (`KismetMathLibrary.BreakVector` (* (`SceneComponent.GetForwardVector` (`self.Arrow`)) (`self.JumpForceValue`))))
  (switch `/Game/Blueprints/JumpPadDirection` (`self.JumpDirection`)
    (:`NewEnumerator0`
      _)
    (:`NewEnumerator1`
      (`SceneComponent.K2_SetRelativeTransform` (`self.Arrow`) (`KismetMathLibrary.MakeTransform` (0.0 50.0 60.0) (struct :`Yaw` 90.0)) false false))
    (:`NewEnumerator2`
      (`SceneComponent.K2_SetRelativeTransform` (`self.Arrow`) (`KismetMathLibrary.MakeTransform` (0.0 -50.0 60.0) (struct :`Yaw` -90.0)) false false))
    (:`NewEnumerator3`
      (`SceneComponent.K2_SetRelativeTransform` (`self.Arrow`) (`KismetMathLibrary.MakeTransform` (-50.0 0.0 60.0) (struct :`Yaw` -180.0)) false false))
    (:`NewEnumerator4`
      (`SceneComponent.K2_SetRelativeTransform` (`self.Arrow`) (`KismetMathLibrary.MakeTransform` (0.0 0.0 110.0) (struct :`Pitch` 90.0)) false false)))
  (set `self.DefinitiveImpulse` (`KismetMathLibrary.MakeVector` _returnvalue_x _returnvalue_y (+ _returnvalue_z (`self.JumpOffset`)))))