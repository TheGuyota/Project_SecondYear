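; TestBuff_BP is a test power-up pickup actor with a Box collider, meant to boost a player stat temporarily.
; Its pickup logic, which is disconnected and never runs, calls the player character's ApplyPowerUpOLD with a multiplier and duration.
; That logic then either destroys the actor or, if static, hides it and disables collision until a timer fires RespawnBuff to restore both.
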(event `RespawnBuff`
  (`self.SetActorHiddenInGame` self false)
  (`PrimitiveComponent.SetCollisionEnabled` (`self.Box`) "QueryAndPhysics"))

(fn `UserConstructionScript`)