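; HP regen power-up that temporarily changes the player's HP regeneration rate.
; PowerUp sets the player's regen multiplier, or replaces the active pickup by destroying it, then starts timers to restore the rate and run a temporary countdown.
; The pickup hides and disables collision on use.
; After the respawn delay it reappears if static, otherwise it destroys itself.
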(event `/Game/Blueprints/Core/PowerUp_Interface.PowerUp`
  (params (PlayerRef :type "/Game/Blueprints/MainCharacter_BP Object Reference"))
  (bind _currenthpregen (`/Game/Blueprints/MainCharacter_BP.CurrentHPRegen` PlayerRef))
  (bind _output_get (set `self.Player Ref` PlayerRef))
  (set `self.CountdownCounter` (`KismetMathLibrary.FTrunc` (`self.PowerUpDuration`)))
  (`/Engine/EditorBlueprintResources/StandardMacros.IsValid` _currenthpregen
    (:`Is Valid`
      (`self.K2_DestroyActor` _currenthpregen))
    (:`Is Not Valid`
      (set `/Game/Blueprints/MainCharacter_BP.HPRegenMultiplier` (`self.TimeBetweenEachRegen`) _output_get)))
  (`/Game/Blueprints/MainCharacter_BP.UpdateHPRegen` _output_get)
  (set `/Game/Blueprints/MainCharacter_BP.CurrentHPRegen` self (`self.Player Ref`))
  (`KismetSystemLibrary.K2_SetTimerDelegate` (delegate `StopPowerUp`) (`self.PowerUpDuration`))
  ;[1 0 0] TEMP
  (`KismetSystemLibrary.K2_SetTimerDelegate` (delegate `Countdown`) 1.0 true)
  (`self.SetActorHiddenInGame` self true)
  (`PrimitiveComponent.SetCollisionEnabled` (`self.Box`) "NoCollision")
  (`KismetSystemLibrary.K2_SetTimerDelegate` (delegate `RespawnOrDestroy`) (`self.SecondsBetweenRespawn`)))

(event `RespawnOrDestroy`
  (if (`self.bIsStatic`)
    (`self.SetActorHiddenInGame` self false)
    (`PrimitiveComponent.SetCollisionEnabled` (`self.Box`) "QueryAndPhysics")
    (else
      (`self.K2_DestroyActor`))))

(event `StopPowerUp`
  (bind _player_ref (`self.Player Ref`))
  (set `/Game/Blueprints/MainCharacter_BP.HPRegenMultiplier` 1.0 _player_ref)
  (`/Game/Blueprints/MainCharacter_BP.UpdateHPRegen` _player_ref)
  (set `/Game/Blueprints/MainCharacter_BP.CurrentHPRegen` null (`self.Player Ref`)))

(event `Countdown`
  (`/Engine/EditorBlueprintResources/StandardMacros.DecrementInt` (`self.CountdownCounter`)))

(fn `UserConstructionScript`
  (`parent.UserConstructionScript`))