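; Jump-boost power-up pickup (BalzoDelConiglio, "rabbit's leap") that temporarily raises the player's JumpZVelocity.
; PowerUp destroys any active instance on the player instead of reapplying the buff, then registers itself and starts timers.
; One timer resets jump velocity to a hardcoded 400; a temporary one ticks a countdown.
; The pickup hides without collision until a respawn timer restores it if static or destroys it.
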(event `/Game/Blueprints/Core/PowerUp_Interface.PowerUp`
  (params (PlayerRef :type "/Game/Blueprints/MainCharacter_BP Object Reference"))
  (bind _currentbalzodelconiglio (`/Game/Blueprints/MainCharacter_BP.CurrentBalzoDelConiglio` PlayerRef))
  (set `self.CountdownCounter` (`KismetMathLibrary.FTrunc` (`self.PowerUpDuration`)))
  (`/Engine/EditorBlueprintResources/StandardMacros.IsValid` _currentbalzodelconiglio
    (:`Is Valid`
      (`self.K2_DestroyActor` _currentbalzodelconiglio))
    (:`Is Not Valid`
      (set `CharacterMovementComponent.JumpZVelocity` (`KismetMathLibrary.Conv_IntToDouble` (`self.BuffedJumpValue`)) (`Character.CharacterMovement` PlayerRef))))
  (set `/Game/Blueprints/MainCharacter_BP.CurrentBalzoDelConiglio` self PlayerRef)
  (`KismetSystemLibrary.K2_SetTimerDelegate` (delegate `StopPowerUp`) (`self.PowerUpDuration`))
  ;[1 0 0] TEMP
  (`KismetSystemLibrary.K2_SetTimerDelegate` (delegate `Countdown`) 1.0 true)
  (`self.SetActorHiddenInGame` self true)
  (`PrimitiveComponent.SetCollisionEnabled` (`self.Box`) "NoCollision")
  (`KismetSystemLibrary.K2_SetTimerDelegate` (delegate `RespawnOrDestroy`) (`self.SecondsBetweenRespawn`)))

(event `StopPowerUp`
  (set `CharacterMovementComponent.JumpZVelocity` 400.0 (`Character.CharacterMovement` (stale `/Game/Blueprints/Core/PowerUp_Interface.PowerUp` PlayerRef)))
  (set `/Game/Blueprints/MainCharacter_BP.CurrentBalzoDelConiglio` null (stale `/Game/Blueprints/Core/PowerUp_Interface.PowerUp` PlayerRef)))

(event `RespawnOrDestroy`
  (if (`self.bIsStatic`)
    (`self.SetActorHiddenInGame` self false)
    (`PrimitiveComponent.SetCollisionEnabled` (`self.Box`) "QueryAndPhysics")
    (else
      (`self.K2_DestroyActor`))))

(event `Countdown`
  (`/Engine/EditorBlueprintResources/StandardMacros.DecrementInt` (`self.CountdownCounter`)))

(fn `UserConstructionScript`
  (`parent.UserConstructionScript`))