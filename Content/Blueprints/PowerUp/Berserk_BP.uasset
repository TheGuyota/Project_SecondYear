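; Berserk power-up Blueprint that temporarily doubles the DMG of the player passed to its PowerUp event.
; It stores the starting DMG and restores it on a timer after PowerUpDuration.
; On use it hides itself and disables its Box collision, then a second timer either respawns it if IsStatic or destroys it.
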(event `/Game/Blueprints/Core/PowerUp_Interface.PowerUp`
  (params (PlayerRef :type "/Game/Blueprints/MainCharacter_BP Object Reference"))
  (bind _dmg (`/Game/Blueprints/MainCharacter_BP.DMG` PlayerRef))
  (set `self.StartingDMG` _dmg)
  (set `/Game/Blueprints/MainCharacter_BP.DMG` (* _dmg 2.0) PlayerRef)
  (`KismetSystemLibrary.K2_SetTimerDelegate` (delegate `StopPowerUp`) (`self.PowerUpDuration`))
  (`self.SetActorHiddenInGame` self true)
  (`PrimitiveComponent.SetCollisionEnabled` (`self.Box`) "NoCollision")
  (`KismetSystemLibrary.K2_SetTimerDelegate` (delegate `RespawnOrDestroy`) (`self.SecondsBetweenRespawn`)))

(event `StopPowerUp`
  (set `/Game/Blueprints/MainCharacter_BP.DMG` (`self.StartingDMG`) (stale `/Game/Blueprints/Core/PowerUp_Interface.PowerUp` PlayerRef)))

(event `RespawnOrDestroy`
  (if (`self.bIsStatic`)
    (`self.SetActorHiddenInGame` self false)
    (`PrimitiveComponent.SetCollisionEnabled` (`self.Box`) "QueryAndPhysics")
    (else
      (`self.K2_DestroyActor`))))

(fn `UserConstructionScript`
  (`parent.UserConstructionScript`))