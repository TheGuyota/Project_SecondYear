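; Shield power-up pickup that adds shield to the player passed into its PowerUp event, capped at that player's maximum.
; On use it hides itself, disables its Box collision and starts a one-shot timer.
; When the timer fires, a static pickup reappears with collision restored, while a non-static one destroys itself.
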(event `/Game/Blueprints/Core/PowerUp_Interface.PowerUp`
  (params (PlayerRef :type "/Game/Blueprints/MainCharacter_BP Object Reference"))
  (bind _shield_max (`/Game/Blueprints/MainCharacter_BP.Shield_Max` PlayerRef))
  (bind _returnvalue (+ (`/Game/Blueprints/MainCharacter_BP.Shield_Current` PlayerRef) (`KismetMathLibrary.Conv_IntToDouble` (`self.ShieldValueToAdd`))))
  (if (> _returnvalue _shield_max)
    (set `/Game/Blueprints/MainCharacter_BP.Shield_Current` _shield_max PlayerRef)
    (else
      (set `/Game/Blueprints/MainCharacter_BP.Shield_Current` _returnvalue PlayerRef)))
  (`self.SetActorHiddenInGame` self true)
  (`PrimitiveComponent.SetCollisionEnabled` (`self.Box`) "NoCollision")
  (`KismetSystemLibrary.K2_SetTimerDelegate` (delegate `RespawnOrDestroy`) (`self.SecondsBetweenRespawn`)))

(event `RespawnOrDestroy`
  (if (`self.bIsStatic`)
    (`self.SetActorHiddenInGame` self false)
    (`PrimitiveComponent.SetCollisionEnabled` (`self.Box`) "QueryAndPhysics")
    (else
      (`self.K2_DestroyActor`))))

(fn `UserConstructionScript`
  (`parent.UserConstructionScript`))