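; PiedeLesto_BP is a speed power-up pickup that temporarily multiplies the player's MaxWalkSpeed.
; On PowerUp it applies the multiplier, hides itself and disables its box collision, then starts separate duration and respawn timers.
; The duration timer resets walk speed to the player's SpeedMax.
; The respawn timer re-shows static pickups with collision restored and destroys non-static ones.
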(event `/Game/Blueprints/Core/PowerUp_Interface.PowerUp`
  (params (PlayerRef :type "/Game/Blueprints/MainCharacter_BP Object Reference"))
  (bind _charactermovement (`Character.CharacterMovement` PlayerRef))
  (set `CharacterMovementComponent.MaxWalkSpeed` (* (`CharacterMovementComponent.MaxWalkSpeed` _charactermovement) (`self.Multiplier`)) _charactermovement)
  (`KismetSystemLibrary.K2_SetTimerDelegate` (delegate `StopPowerUp`) (`self.PowerUpDuration`))
  (`self.SetActorHiddenInGame` self true)
  (`PrimitiveComponent.SetCollisionEnabled` (`self.Box`) "NoCollision")
  (`KismetSystemLibrary.K2_SetTimerDelegate` (delegate `RespawnOrDestroy`) (`self.SecondsBetweenRespawn`)))

(event `RespawnOrDestroy`
  (if (`self.bIsStatic`)
    (`self.SetActorHiddenInGame` self false)
    (`PrimitiveComponent.SetCollisionEnabled` (`self.Box`) "QueryAndPhysics")
    (else
      (`self.K2_DestroyActor`))))

(event `StopPowerUp`
  (set `CharacterMovementComponent.MaxWalkSpeed` (`/Game/Blueprints/MainCharacter_BP.SpeedMax` (stale `/Game/Blueprints/Core/PowerUp_Interface.PowerUp` PlayerRef)) (`Character.CharacterMovement` (stale `/Game/Blueprints/Core/PowerUp_Interface.PowerUp` PlayerRef))))

(fn `UserConstructionScript`
  (`parent.UserConstructionScript`))